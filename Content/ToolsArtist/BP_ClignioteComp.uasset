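; Blink actor that pulses the intensity of a referenced Lamp light between max and min, starting on BeginPlay.
; Clignote plays one timeline forward from start or in reverse depending on the On flag, with a separate speed setting for each direction.
; The timeline track drives the intensity Lerp, and its Finished pin re-calls Clignote before flipping On, so each flip takes effect one pass later.
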(event Custom|Clignote
  (if (Variables|Default|GetOn)
    (Components|Timeline|SetPlayRate (Variables|Default|GetCligonteTimeLigne) (/ 1.0 (Variables|Default|GetClignoteSpeedOFF)))
    (bind _newtrack_0 (Timeline|CligonteTimeLigne PlayFromStart)
      (:Update
        (Rendering|Components|Light|SetIntensity (Variables|/Script/Engine.Light|GetLightComponent (Variables|Default|GetLamp)) (Math|Float|Lerp (Variables|Default|GetIntensityMax) (Variables|Default|GetIntensityMin) _newtrack_0)))
      (:Finished
        (CallFunction|Clignote)
        (Variables|Default|SetOn (not (Variables|Default|GetOn)))))
    (else
      (Components|Timeline|SetPlayRate (Variables|Default|GetCligonteTimeLigne) (/ 1.0 (Variables|Default|GetClignoteSpeedON)))
      (Timeline|CligonteTimeLigne Reverse))))

(event EventBeginPlay
  (CallFunction|Clignote))

(fn ConstructionScript)