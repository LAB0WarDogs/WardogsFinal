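; Second playable character, a child Blueprint that specializes the parent's three skill slots with melee attack, PouettePouette and grenade skill components.
; Skill overrides call the parent, then forward to components: melee fires on activation, while the other two activate first and fire through UseFirstSkill.
; Cancellation targets the active skill's component.
; After a short BeginPlay delay, it binds inventory battery use and loops a timer updating the camera's health vignette.
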(event Custom|vignette
  ;[0 0 1] Comment
  (CallFunction|VignettePercentage (Variables|Default|GetHealth) (Variables|Default|GetCamera)))

(event Custom|UsingBattery-SecondChara
  ;[0 0 1] Comment
  (CallFunction|UseBattery))

(event EventBeginPlay
  ;[0 0 1] Comment
  (Utilities|FlowControl|Delay 0.2)
  (Utilities|FlowControl|Sequence
    (:then_0
      (|CallParentFunction)
      (bind _ascharacter_master (CallFunction|GetPlayerCharacterMaster))
      (EventDispatchers|BindEventtoUseBatteryfromInventory _ascharacter_master (delegate Custom|UsingBattery-SecondChara)))
    (:then_1
      (Utilities|Time|SetTimerbyEvent (delegate Custom|vignette) 0.1 true))))

(event EventTakeDamage
  (params (Damage :type Float%20%28double-precision%29))
  ;[0 0 1] Take Damage
  (CallFunction|TakeDamagefromEnnemyorFriend Damage))

(fn ConstructionScript
  (|CallParentFunction))

(fn UseBattery
  (|CallParentFunction))

(fn ActivateFirstSkill
  (|CallParentFunction)
  (Default|UseFirstSkill (Variables|Default|GetBP_MeleeAttack)))

(fn UseFirstSkill
  (params (FirstSkillActive? :type Boolean) (SecondSkillActive? :type Boolean) (ThirdSkillActive? :type Boolean))
  (|CallParentFunction FirstSkillActive? SecondSkillActive? ThirdSkillActive?)
  (if SecondSkillActive?
    (Default|UsingSegondSkill (Variables|Default|GetBP_PouettePouetteSkill))
    (elif ThirdSkillActive?
      (Default|UsingThirdSkill (Variables|Default|GetBP_Grenade)))))

(fn ActivateSecondSkill
  (|CallParentFunction)
  (Default|ActivatSegondSkill (Variables|Default|GetBP_PouettePouetteSkill)))

(fn ActivateThirdSkill
  (|CallParentFunction)
  (Default|ActivateThirdSkill (Variables|Default|GetBP_Grenade)))

(fn GetHealth
  (params (DamageTaken :type Float%20%28double-precision%29))
  (|CallParentFunction DamageTaken))

(fn TakeDamagefromEnnemyorFriend
  (params (DamageTaken :type Float%20%28double-precision%29))
  (|CallParentFunction DamageTaken))

(fn CancelSkill
  (params (FirstSkillActive? :type Boolean) (SecondSkillActive? :type Boolean) (ThirdSkillActive? :type Boolean))
  (|CallParentFunction FirstSkillActive? SecondSkillActive? ThirdSkillActive?)
  (if FirstSkillActive?
    (Default|Cancelation (Variables|Default|GetBP_MeleeAttack))
    (elif SecondSkillActive?
      (Default|Cancelation (Variables|Default|GetBP_PouettePouetteSkill))
      (elif ThirdSkillActive?
        (Default|Cancelation (Variables|Default|GetBP_Grenade))))))