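; First playable character Blueprint: a sniper with Sniper, Flair and Camouflage skills.
; Skill overrides call the parent, then forward to the matching skill components.
; Timelines drive aim sway, camera zoom, stealth material parameters and grappling-hook travel, which locks input and character switching.
; Looping timers update the health vignette, cable end, electric arc and trace-clipped laser pointer, while damage blends the view to this character.
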(event Custom|ElectricArc
  (bind _snipercomptarget (Variables|Default|GetSniperCompTarget))
  (bind _returnvalue (Transformation|GetWorldLocation _snipercomptarget))
  ;[0 0 1] Electric Arc VFX
  (Effects|Components|ParticleSystem|SetVectorParameter (Variables|Default|GetNS_ElectricArc) "User.BeamEnd" _returnvalue)
  (Effects|Components|ParticleSystem|SetVectorParameter (Variables|Default|GetNS_Sparks) "User.Orientation" (.location (Class|KismetAnimationLibrary|Lookat (Transformation|GetWorldTransform _snipercomptarget) _returnvalue (Transformation|GetWorldLocation (Variables|Default|GetStartingPoint)) true "0, 0, 0" 0.0))))

(event Custom|CursorMovement
  (Utilities|FlowControl|Sequence
    (:then_0
      (Components|Timeline|SetPlayRate (Variables|Default|GetTL_CursorMovement) (/ 1.0 (Math|Random|RandomFloatinRange 1.5 2.0)))
      (bind _sinus (Timeline|TL_CursorMovement Play)
        (:Update
          (Variables|/Game/Blueprint/SkiilsActorComponent/BP_SniperSkill.BP_SniperSkill_C|SetAlpha (Variables|Default|GetBP_SniperSkill) _sinus))))
    (:then_1
      (Components|Timeline|SetPlayRate (Variables|Default|GetTimeline_0) (/ 1.0 (Math|Random|RandomFloatinRange 1.5 2.0)))
      (bind _sinus_2 (Timeline|Timeline_0 Play)
        (:Update
          (Variables|/Game/Blueprint/SkiilsActorComponent/BP_SniperSkill.BP_SniperSkill_C|SetAlpha_0 (Variables|Default|GetBP_SniperSkill) _sinus_2))))))

(event Custom|HideSniper
  ;[0 0 1] Set Sniper Visibility
  (Rendering|SetVisibility (Variables|Default|GetArme_sniper) false false)
  (Rendering|SetVisibility (Variables|Default|GetSniperIdle) true false))

(event Custom|StartElectricArc
  ;[0 0 1] Electric Arc VFX
  (bind _returnvalue (Utilities|Time|SetTimerbyEvent (delegate Custom|ElectricArc) 0.1 true))
  (Variables|Default|SetElectricArcTimer _returnvalue))

(event Custom|StopElectricArc
  ;[0 0 1] Electric Arc VFX
  (Utilities|Time|ClearandInvalidateTimerbyHandle (Variables|Default|GetElectricArcTimer)))

(event Custom|StartLaserAimAssist
  ;[0 0 1] Laser Pointer VFX
  (bind _returnvalue (Utilities|Time|SetTimerbyEvent (delegate Custom|LaserPointer) 0.001 true))
  (Variables|Default|SetLaserPointerTimer _returnvalue))

(event Custom|LaserPointer
  ;[0 0 1] Laser Pointer VFX
  (bind (_outhit _returnvalue) (Collision|LineTraceByChannel (Transformation|GetWorldLocation (Variables|Default|GetStartingPoint)) (Transformation|GetWorldLocation (Variables|Default|GetSniperCompTarget)) "TraceTypeQuery6" false 0 "None"))
  (if _returnvalue
    (Effects|Components|ParticleSystem|SetVectorParameter (Variables|Default|GetNS_LaserPointer) "User.BeamEnd" (.Location (Collision|BreakHitResult _outhit)))
    (else
      (Effects|Components|ParticleSystem|SetVectorParameter (Variables|Default|GetNS_LaserPointer) "User.BeamEnd" (Transformation|GetWorldLocation (Variables|Default|GetSniperCompTarget))))))

(event Custom|StopLaserPointer
  ;[0 0 1] Laser Pointer VFX
  (Utilities|Time|ClearandInvalidateTimerbyHandle (Variables|Default|GetLaserPointerTimer)))

(event Custom|vignette
  ;[0 0 1] Comment
  (CallFunction|VignettePercentage (Variables|Default|GetHealth) (Variables|Default|GetCamera)))

(event Custom|ShowSniper
  ;[0 0 1] Set Sniper Visibility
  (Rendering|SetVisibility (Variables|Default|GetArme_sniper) true false)
  (Rendering|SetVisibility (Variables|Default|GetSniperIdle) false false))

(event Custom|UsingCamo
  ;[0 0 1] Timeline Camo
  (bind (_direction _opacity _normal_depth) (Timeline|Timeline_0_0 PlayFromStart)
    (:Update
      (Rendering|Material|SetScalarParameterValue "/Game/Material/Stealth/MPC_Stealth.MPC_Stealth" "Opacity" _opacity :!class /Script/Engine.KismetMaterialLibrary)
      (Rendering|Material|SetScalarParameterValue "/Game/Material/Stealth/MPC_Stealth.MPC_Stealth" "Normal Depth" _normal_depth :!class /Script/Engine.KismetMaterialLibrary))))

(event Custom|Zoom
  ;[0 0 1] Timeline Zoom Dezoom
  (Components|Timeline|SetPlayRate (Variables|Default|GetZoomDezoomTL) (/ 1.0 (Variables|Default|GetZoomDezoomTimeSniperSkill)))
  (bind _zoom_dezoom (Timeline|ZoomDezoomTL Play)
    (:Update
      (Variables|/Script/Engine.SpringArmComponent|SetTargetArmLength (Variables|Default|GetSpringArm) (Math|Float|Lerp 1.6e+03 1.8e+03 _zoom_dezoom)))))

(event Custom|Dezoom
  ;[0 0 1] Timeline Zoom Dezoom
  (bind _zoom_dezoom (Timeline|ZoomDezoomTL Reverse)
    (:Update
      (Variables|/Script/Engine.SpringArmComponent|SetTargetArmLength (Variables|Default|GetSpringArm) (Math|Float|Lerp 1.6e+03 1.8e+03 _zoom_dezoom)))))

(event Custom|StopUsingCamo
  ;[0 0 1] Timeline Camo
  (bind (_direction _opacity _normal_depth) (Timeline|Timeline_0_0 Reverse)
    (:Update
      (Rendering|Material|SetScalarParameterValue "/Game/Material/Stealth/MPC_Stealth.MPC_Stealth" "Opacity" _opacity :!class /Script/Engine.KismetMaterialLibrary)
      (Rendering|Material|SetScalarParameterValue "/Game/Material/Stealth/MPC_Stealth.MPC_Stealth" "Normal Depth" _normal_depth :!class /Script/Engine.KismetMaterialLibrary))))

(event Custom|UseBattery-FirstChara
  ;[0 0 1] Comment
  (if (Variables|/Game/Blueprint/SkiilsActorComponent/BP_Camouflage.BP_Camouflage_C|GetSkillIsBeingUsed? (Variables|Default|GetBP_Camouflage))
    (CallFunction|UseBattery)))

(event Custom|MovePlayerAlongGrapple
  (bind _as_game_mode_wardogs (Variables|Default|GetAs%20Game%20Mode%20Wardogs))
  (bind _as_game_mode_wardogs_2 (Variables|Default|GetAs%20Game%20Mode%20Wardogs))
  ;[0 0 1] Move the player along the grappling hook
  (Utilities|IsValid _as_game_mode_wardogs
    (:Is%20Valid
      (Variables|/Game/Blueprint/GameMode/GameModeWardogs.GameModeWardogs_C|SetCanSwitch _as_game_mode_wardogs false)
      (Variables|Default|SetIsUsingSkill true)
      (Input|DisableInput (Game|GetPlayerController 0) 0)
      (Components|Timeline|SetPlayRate (Variables|Default|GetMovePlayer) (/ 1.0 (Math|Float|Clamp(Float) (/ (Math|Vector|VectorLength (- (Variables|Default|GetGrappleEndLocation) (Variables|Default|GetGrappleStartLocation))) 1.2e+03) 1.0 5.0)))
      (bind _returnvalue (Utilities|Time|SetTimerbyEvent (delegate Custom|SetGrapplingHookEndLocaton) 0.01 true))
      (Pawn|Components|CharacterMovement|DisableMovement (Variables|Character|GetCharacterMovement))
      (Variables|Default|SetIsUsingGrapplingHook true)
      (Utilities|FlowControl|Delay 0.5)
      (Rendering|SetVisibility (Variables|Default|GetCable) true false)
      (CallFunction|HideSniper)
      (Utilities|FlowControl|Delay 0.2)
      (bind _grapplingtrack (Timeline|MovePlayer PlayFromStart)
        (:Update
          (Transformation|SetActorLocation (Math|Vector|Lerp(Vector) (Variables|Default|GetGrappleStartLocation) (Variables|Default|GetGrappleEndLocation) _grapplingtrack) false false))
        (:Finished
          (Pawn|Components|CharacterMovement|SetMovementMode (Variables|Character|GetCharacterMovement) "MOVE_Walking" 0)
          (Utilities|Time|ClearandInvalidateTimerbyHandle _returnvalue)
          (Rendering|SetVisibility (Variables|Default|GetCable) false false)
          (Variables|Default|SetIsUsingSkill false)
          (Variables|Default|SetIsUsingGrapplingHook false)
          (CallFunction|ShowSniper)
          (Utilities|IsValid _as_game_mode_wardogs_2
            (:Is%20Valid
              (Variables|/Game/Blueprint/GameMode/GameModeWardogs.GameModeWardogs_C|SetCanSwitch _as_game_mode_wardogs_2 true)
              (Input|EnableInput (Game|GetPlayerController 0) 0))))))))

(event Custom|SetGrapplingHookEndLocaton
  ;[0 0 1] Move the player along the grappling hook
  (Variables|/Script/CableComponent.CableComponent|SetEndLocation (Variables|Default|GetCable) (Math|Transform|InverseTransformLocation (Transformation|GetActorTransform) (Variables|Default|GetGrappleEndLocation))))

(event EventBeginPlay
  ;[0 0 1] Comment
  (Utilities|FlowControl|Delay 0.2)
  (Utilities|FlowControl|Sequence
    (:then_0
      (|CallParentFunction)
      (bind _ascharacter_master (Utilities|Casting|CastToCharacterMaster (Game|GetPlayerCharacter 0)))
      (Variables|Default|SetAs%20Character%20Master _ascharacter_master)
      (EventDispatchers|BindEventtoUseBatteryfromInventory _ascharacter_master (delegate Custom|UseBattery-FirstChara))
      (bind _asgame_mode_wardogs (CallFunction|GetGameMode))
      (Variables|Default|SetAs%20Game%20Mode%20Wardogs _asgame_mode_wardogs))
    (:then_1
      (Utilities|Time|SetTimerbyEvent (delegate Custom|vignette) 0.1 true))))

(event EventTakeDamage
  (params (Damage :type Float%20%28double-precision%29))
  ;[0 0 1] Take Damage
  (CallFunction|TakeDamagefromEnnemyorFriend Damage))

(fn ConstructionScript
  (|CallParentFunction))

(fn ActivateFirstSkill
  (|CallParentFunction)
  (Default|ActivateSniperSkill (Variables|Default|GetBP_SniperSkill)))

(fn UseFirstSkill
  (params (FirstSkillActive? :type Boolean) (SecondSkillActive? :type Boolean) (ThirdSkillActive? :type Boolean))
  (|CallParentFunction FirstSkillActive? SecondSkillActive? ThirdSkillActive?)
  (if FirstSkillActive?
    (Default|UseSniperSkill (Variables|Default|GetBP_SniperSkill))))

(fn ActivateSecondSkill
  (|CallParentFunction)
  (Default|ActivateSecondSkill (Variables|Default|GetBP_FlairSkill)))

(fn UseBattery
  (|CallParentFunction))

(fn ActivateThirdSkill
  (|CallParentFunction)
  (Default|ActivateThirdSkill (Variables|Default|GetBP_Camouflage)))

(fn GetHealth
  (params (DamageTaken :type Float%20%28double-precision%29))
  (|CallParentFunction DamageTaken))

(fn TakeDamagefromEnnemyorFriend
  (params (DamageTaken :type Float%20%28double-precision%29))
  (Game|Player|SetViewTargetwithBlend (Game|GetPlayerController 0) (Variables|Default|GetFirstChara) 0.0 "VTBlend_Linear" 0.0 true)
  (|CallParentFunction DamageTaken))

(fn CancelSkill
  (params (FirstSkillActive? :type Boolean) (SecondSkillActive? :type Boolean) (ThirdSkillActive? :type Boolean))
  (|CallParentFunction FirstSkillActive? SecondSkillActive? ThirdSkillActive?)
  (if FirstSkillActive?
    (Default|Cancelation (Variables|Default|GetBP_SniperSkill))
    (elif (not SecondSkillActive?)
      (if ThirdSkillActive?
        (Default|Cancelation (Variables|Default|GetBP_Camouflage))))))