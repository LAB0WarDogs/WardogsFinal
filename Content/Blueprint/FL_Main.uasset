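; FL_Main is a function library of shortcut getters for the game's core player and framework objects.
; Each function fetches an engine object and returns it cast to the project class: CharacterMaster, MyPlayerController, GameModeWardogs or BP_Drone.
; Player lookups always use index 0, and the drone getter succeeds only when that player's pawn is a BP_Drone.
; A failed cast returns no object.
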(fn GetPlayerCharacterMaster
  (bind _ascharacter_master (Utilities|Casting|CastToCharacterMaster (Game|GetPlayerCharacter 0))
    (:then
      (return _ascharacter_master))
    (:CastFailed
      (return 0))))

(fn GetPlayerController
  (bind _asmy_player_controller (Utilities|Casting|CastToMyPlayerController (Game|GetPlayerController 0))
    (:then
      (return _asmy_player_controller))
    (:CastFailed
      (return 0))))

(fn GetGameMode
  (bind _asgame_mode_wardogs (Utilities|Casting|CastToGameModeWardogs (Game|GetGameMode))
    (:then
      (return _asgame_mode_wardogs))
    (:CastFailed
      (return 0))))

(fn GetDrone
  (bind _asbp_drone (Utilities|Casting|CastToBP_Drone (Game|Player|GetPlayerPawn 0))
    (:then
      (return _asbp_drone))
    (:CastFailed
      (return 0))))