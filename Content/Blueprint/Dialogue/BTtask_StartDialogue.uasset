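; Behavior tree task that opens a dialogue box on the Wardogs game mode's HUD and stores it in the blackboard along with the cinematic flag.
; In cinematic mode it recreates the HUD, shows the mid-screen box, disables player input and hides the in-game UI.
; Otherwise it claims the first of two boxes that is not visible, retrying every half second while both are busy, then finishes successfully.
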(event EventReceiveExecuteAI
  (params (OwnerController :type AI%20Controller%20Object%20Reference) (ControlledPawn :type Pawn%20Object%20Reference))
  (bind _returnvalue (Game|GetPlayerController 0))
  (bind _cinematique (Variables|Default|GetCinematique))
  ;[0 1 0] Start Dialogue System
  (bind _asgame_mode_wardogs (Utilities|Casting|CastToGameModeWardogs (Game|GetGameMode)))
  (Class|BTFunctionLibrary|SetBlackboardValueasBool (Variables|Default|GetBB_Cinematique) _cinematique)
  (if _cinematique
    (Widget|RemovefromParent (Variables|/Game/Blueprint/GameMode/GameModeWardogs.GameModeWardogs_C|GetHeadUpDisplay _asgame_mode_wardogs))
    (bind _returnvalue_2 (UserInterface|CreateWidget "/Game/UI/Dialogue/HeadUpDisplay.HeadUpDisplay_C"))
    (bind _output_get (Variables|/Game/Blueprint/GameMode/GameModeWardogs.GameModeWardogs_C|SetHeadUpDisplay _asgame_mode_wardogs _returnvalue_2))
    ;;[0 0 0] Text in Mid Screen
    (UserInterface|Viewport|AddtoViewport _output_get 0)
    (Widget|SetVisibility (Variables|/Game/UI/Dialogue/HeadUpDisplay.HeadUpDisplay_C|GetDialogueBox_40 _output_get) "Visible")
    (Class|BTFunctionLibrary|SetBlackboardValueasObject (Variables|Default|GetBB_DialogueUI) (Variables|/Game/UI/Dialogue/HeadUpDisplay.HeadUpDisplay_C|GetDialogueBox_40 _output_get))
    (Input|DisableInput _returnvalue _returnvalue)
    (bind _asgame_mode_wardogs_2 (CallFunction|GetGameMode))
    (Widget|SetIsEnabled (Variables|/Game/Blueprint/GameMode/GameModeWardogs.GameModeWardogs_C|GetInGameUI _asgame_mode_wardogs_2) false)
    (Widget|SetVisibility (Variables|/Game/Blueprint/GameMode/GameModeWardogs.GameModeWardogs_C|GetInGameUI _asgame_mode_wardogs_2) "Hidden")
    (else
      (if (Utilities|Enum|NotEqual(Enum) (Widget|GetVisibility (Variables|/Game/UI/Dialogue/HeadUpDisplay.HeadUpDisplay_C|GetDialogueBox _output_get)) "Visible") :!label _label
        ;;[0 0 0] Text in Top Screen
        (Widget|SetVisibility (Variables|/Game/UI/Dialogue/HeadUpDisplay.HeadUpDisplay_C|GetDialogueBox _output_get) "Visible")
        (Class|BTFunctionLibrary|SetBlackboardValueasObject (Variables|Default|GetBB_DialogueUI) (Variables|/Game/UI/Dialogue/HeadUpDisplay.HeadUpDisplay_C|GetDialogueBox _output_get))
        (elif (Utilities|Enum|NotEqual(Enum) (Widget|GetVisibility (Variables|/Game/UI/Dialogue/HeadUpDisplay.HeadUpDisplay_C|GetDialogueBox_1 _output_get)) "Visible")
          (Widget|SetVisibility (Variables|/Game/UI/Dialogue/DialogueBox.DialogueBox_C|GetBorderIcone (Variables|/Game/UI/Dialogue/HeadUpDisplay.HeadUpDisplay_C|GetDialogueBox_1 _output_get)) "Visible")
          (Class|BTFunctionLibrary|SetBlackboardValueasObject (Variables|Default|GetBB_DialogueUI) (Variables|/Game/UI/Dialogue/HeadUpDisplay.HeadUpDisplay_C|GetDialogueBox_1 _output_get))
          (else
            (Utilities|FlowControl|Delay 0.5)
            (goto _label))))))
  (AI|BehaviorTree|FinishExecute true))