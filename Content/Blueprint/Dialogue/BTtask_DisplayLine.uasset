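; Behavior tree task that displays one dialogue line in the DialogueBox widget stored on the blackboard.
; On execute it sets the text, speaker name and portrait texture on the widget.
; When the Cinematique blackboard flag is set, Droite chooses which image and name borders are visible.
; On tick it finishes successfully when a key bound to the Interact action is pressed, letting the tree advance.
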(event EventReceiveExecuteAI
  (params (OwnerController :type AI%20Controller%20Object%20Reference) (ControlledPawn :type Pawn%20Object%20Reference))
  ;[0 1 0] Set text
  (bind _asdialogue_box (Utilities|Casting|CastToDialogueBox (Class|BTFunctionLibrary|GetBlackboardValueasObject (Variables|Default|GetDialogueWidget))))
  (Variables|/Game/UI/Dialogue/DialogueBox.DialogueBox_C|SetDialogueText _asdialogue_box (Variables|Default|GetText))
  (Variables|/Game/UI/Dialogue/DialogueBox.DialogueBox_C|SetInterlocuteur _asdialogue_box (Variables|Default|GetInterprête))
  (Appearance|SetBrushfromTexture (Variables|/Game/UI/Dialogue/DialogueBox.DialogueBox_C|GetImageProfile _asdialogue_box) (Variables|Default|GetTexture) false)
  (if (Class|BTFunctionLibrary|GetBlackboardValueasBool (Variables|Default|GetCinematique))
    (if (Variables|Default|GetDroite)
      (Widget|SetVisibility (Variables|/Game/UI/Dialogue/DialogueBox.DialogueBox_C|GetBorderImage_1 _asdialogue_box) "Visible")
      (Widget|SetVisibility (Variables|/Game/UI/Dialogue/DialogueBox.DialogueBox_C|GetBorderImage _asdialogue_box) "Hidden")
      (else
        (Widget|SetVisibility (Variables|/Game/UI/Dialogue/DialogueBox.DialogueBox_C|GetBorderName _asdialogue_box) "Visible")
        (Widget|SetVisibility (Variables|/Game/UI/Dialogue/DialogueBox.DialogueBox_C|GetBorderImage_1 _asdialogue_box) "Hidden")))))

(event EventTick
  (params (OwnerActor :type Actor%20Object%20Reference) (DeltaSeconds :type Float%20%28single-precision%29))
  ;[0 1 0] skip to next text
  (if (Game|Player|WasInputKeyJustPressed (Game|GetPlayerController 0) "AnyKey")
    (for _array_element (Class|InputSettings|GetActionMappingbyName (Class|InputSettings|GetInputSettings) "Interact")
      (if (Game|Player|WasInputKeyJustPressed (Game|GetPlayerController 0) (.Key (Utilities|Struct|BreakInputActionKeyMapping _array_element)))
        (AI|BehaviorTree|FinishExecute true)))))