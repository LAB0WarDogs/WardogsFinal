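; Behavior tree task that ends a dialogue with an AI and returns control to the player.
; On AI execution it hides the dialogue widget stored in the blackboard and re-enables input for the first player controller.
; It then calls EndDialogue on the BP_Test_AI owner controller and shows and enables the game mode's in-game UI before finishing successfully.
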(event EventReceiveExecuteAI
  (params (OwnerController :type AI%20Controller%20Object%20Reference) (ControlledPawn :type Pawn%20Object%20Reference))
  (bind _returnvalue (Game|GetPlayerController 0))
  ;[0 1 0] End dialogue System
  (bind _aswidget (Utilities|Casting|CastToWidget (Class|BTFunctionLibrary|GetBlackboardValueasObject (Variables|Default|GetDialogueWidget))))
  (Widget|SetVisibility _aswidget "Hidden")
  (Input|EnableInput _returnvalue _returnvalue)
  (bind _asbp_test_ai (Utilities|Casting|CastToBP_Test_AI OwnerController))
  (Default|EndDialogue _asbp_test_ai)
  (bind _asgame_mode_wardogs (CallFunction|GetGameMode))
  (Widget|SetIsEnabled (Variables|/Game/Blueprint/GameMode/GameModeWardogs.GameModeWardogs_C|GetInGameUI _asgame_mode_wardogs) true)
  (Widget|SetVisibility (Variables|/Game/Blueprint/GameMode/GameModeWardogs.GameModeWardogs_C|GetInGameUI _asgame_mode_wardogs) "Visible")
  (AI|BehaviorTree|FinishExecute true))