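; BP_AI_Chat is an AI enemy character that deals area damage when a CharacterMaster enters its Sphere component.
; That overlap calls AttackPlayer, which runs a sphere overlap around the AI, ignoring itself, and sends heavy fixed damage to every actor implementing BPI_Damageable.
; BeginPlay, ChangeState and construction defer to the parent class, while TakeDamage calls the parent with zero damage.
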(event OnComponentBeginOverlap(Sphere)
  (params (OverlappedComponent :type Primitive%20Component%20Object%20Reference) (OtherActor :type Actor%20Object%20Reference) (OtherComp :type Primitive%20Component%20Object%20Reference) (OtherBodyIndex :type Integer) (bFromSweep :type Boolean) (SweepResult :type Hit%20Result%20Structure%20%28by%20ref%29))
  (Utilities|Casting|CastToCharacterMaster OtherActor)
  (CallFunction|AttackPlayer))

(event Custom|AttackPlayer
  (bind _outactors (Collision|SphereOverlapActors (Transformation|GetActorLocation) 2.5e+02 (Variables|Default|GetObject%20Types) 0 (Utilities|Array|MakeArray self)))
  (for _array_element _outactors
    (if (Utilities|DoesObjectImplementInterface _array_element "/Game/Blueprint/Interface/BPI_Damageable.BPI_Damageable_C")
      (Class|BPIDamageable|TakeDamage(Message) _array_element 1.1e+02))))

(event EventChangeState
  (params (AlertState :type E_AiStates%20Enum :default "NewEnumerator1"))
  (|CallParentFunction AlertState))

(event EventTakeDamage
  (params (Damage :type Float%20%28double-precision%29))
  (|CallParentFunction 0.0))

(event EventBeginPlay
  (|CallParentFunction))

(fn ConstructionScript
  (|CallParentFunction))