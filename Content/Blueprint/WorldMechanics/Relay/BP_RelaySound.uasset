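; BP_RelaySound is an interactable relay that signals a rise in AI melee attack loudness and can be temporarily disabled.
; Sphere1 overlaps show or hide a widget for CharacterMaster.
; Begin and end overlaps by BP_AI_PucesSentinel or any other non-character actor call RiseAiMeleeAttackLoudness.
; Interact switches off the sphere's collision, then restores query-only collision after a retriggerable five-second delay, printing both states.
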(event OnComponentBeginOverlap(Sphere1)
  (params (OverlappedComponent :type Primitive%20Component%20Object%20Reference) (OtherActor :type Actor%20Object%20Reference) (OtherComp :type Primitive%20Component%20Object%20Reference) (OtherBodyIndex :type Integer) (bFromSweep :type Boolean) (SweepResult :type Hit%20Result%20Structure%20%28by%20ref%29))
  (Utilities|Casting|CastToBP_AI_PucesSentinel OtherActor
    (:then
      (Default|CallRiseAiMeleeAttackLoudness :!label _label))
    (:CastFailed
      (Utilities|Casting|CastToCharacterMaster OtherActor
        (:then
          (Rendering|SetVisibility (Variables|Default|GetWidget) true false))
        (:CastFailed
          (goto _label))))))

(event OnComponentEndOverlap(Sphere1)
  (params (OverlappedComponent :type Primitive%20Component%20Object%20Reference) (OtherActor :type Actor%20Object%20Reference) (OtherComp :type Primitive%20Component%20Object%20Reference) (OtherBodyIndex :type Integer))
  (Utilities|Casting|CastToBP_AI_PucesSentinel OtherActor
    (:then
      (Default|CallRiseAiMeleeAttackLoudness :!label _label))
    (:CastFailed
      (Utilities|Casting|CastToCharacterMaster OtherActor
        (:then
          (Rendering|SetVisibility (Variables|Default|GetWidget) false false))
        (:CastFailed
          (goto _label))))))

(event EventInteract
  (Collision|SetCollisionEnabled (Variables|Default|GetSphere1) "NoCollision")
  (Development|PrintString "Relay Disabled")
  (Utilities|FlowControl|RetriggerableDelay 5.0)
  (Collision|SetCollisionEnabled (Variables|Default|GetSphere1) "QueryOnly")
  (Development|PrintString "Relay Enabled"))

(fn ConstructionScript)