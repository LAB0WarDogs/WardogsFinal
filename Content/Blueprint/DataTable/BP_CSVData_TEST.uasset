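; Test Blueprint that builds a grid of tiles from a data table in its construction script, using two instanced static mesh components.
; Each table row name doubles as a column name, and that column's values are read as numbers.
; Non-zero cells become instances spaced by their indices, with height and vertical scale driven by the value.
; A positive remainder modulo two selects Tile_2; other values use Tile.
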(event EventBeginPlay)

(fn ConstructionScript
  (bind _table (Variables|Default|GetTable))
  (bind _returnvalue (AddComponent|AddHierarchicalInstancedStaticMeshComponent false))
  (bind _output_get (Variables|Default|SetHISM _returnvalue))
  (Components|StaticMesh|SetStaticMesh _output_get "/Game/Blueprint/DataTable/Tile.Tile")
  (bind _returnvalue_2 (AddComponent|AddHierarchicalInstancedStaticMeshComponent false))
  (bind _output_get_2 (Variables|Default|SetHISM_0 _returnvalue_2))
  (Components|StaticMesh|SetStaticMesh _output_get_2 "/Game/Blueprint/DataTable/Tile_2.Tile_2")
  (bind _outrownames (DataTable|GetDataTableRowNames _table))
  (for (_array_element _array_index) _outrownames
    (bind _returnvalue_3 (Class|DataTableFunctionLibrary|GetDataTableColumnasString _table _array_element))
    (for (_array_element_2 _array_index_2) _returnvalue_3
      (if (!= (Math|Conversions|ToFloat(Integer) _array_element_2) 0.0)
        (if (> (Math|Float|%(Float) (Math|Conversions|ToFloat(Integer) _array_element_2) 2.0) 0.0)
          (Components|InstancedStaticMesh|AddInstance (Variables|Default|GetHISM_0) (Math|Transform|MakeTransform (Math|Vector|MakeVector (* (Math|Conversions|ToFloat(Integer) _array_index) 5e+02) (* (Math|Conversions|ToFloat(Integer) _array_index_2) 5e+02) (* (Math|Conversions|ToFloat(Integer) _array_element_2) 1e+02)) (Math|Rotator|MakeRotator 0.0 0.0 0.0) (Math|Vector|MakeVector 1.0 1.0 (Math|Conversions|ToFloat(Integer) _array_element_2))))
          (else
            (Components|InstancedStaticMesh|AddInstance (Variables|Default|GetHISM) (Math|Transform|MakeTransform (Math|Vector|MakeVector (* (Math|Conversions|ToFloat(Integer) _array_index) 5e+02) (* (Math|Conversions|ToFloat(Integer) _array_index_2) 5e+02) (* (Math|Conversions|ToFloat(Integer) _array_element_2) 1e+02)) (Math|Rotator|MakeRotator 0.0 0.0 0.0) (Math|Vector|MakeVector 1.0 1.0 (Math|Conversions|ToFloat(Integer) _array_element_2))))))))))