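; BP_CSVData is a Blueprint that places cube instances at positions read from a data table with X, Y and Z columns.
; Its construction script adds a hierarchical instanced static mesh component and sets its mesh through a random MultiGate, whose three outputs all use the same Cube.
; It then loops over the table rows, adding one unrotated, unit-scale instance at each row's coordinates.
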(event EventBeginPlay)

(fn ConstructionScript
  (bind _table (Variables|Default|GetTable))
  (bind _returnvalue (AddComponent|AddHierarchicalInstancedStaticMeshComponent false))
  (bind _output_get (Variables|Default|SetHISM _returnvalue))
  (Utilities|FlowControl|MultiGate true true -1
    (:Out%200
      (Components|StaticMesh|SetStaticMesh _output_get "/Engine/EngineMeshes/Cube.Cube"))
    (:Out%201
      (Components|StaticMesh|SetStaticMesh _output_get "/Engine/EngineMeshes/Cube.Cube"))
    (:Out%202
      (Components|StaticMesh|SetStaticMesh _output_get "/Engine/EngineMeshes/Cube.Cube")))
  (bind _outrownames (DataTable|GetDataTableRowNames _table))
  (for _array_element _outrownames
    (bind _returnvalue_2 (Utilities|GetDataTableRow _table _array_element)
      (:then
        (bind _output_get_2 (Variables|Default|SetX (.X (Utilities|Struct|BreakS_Demo _returnvalue_2))))
        (bind _output_get_3 (Variables|Default|SetY (.Y (Utilities|Struct|BreakS_Demo _returnvalue_2))))
        (bind _output_get_4 (Variables|Default|SetZ (.Z (Utilities|Struct|BreakS_Demo _returnvalue_2))))
        (Components|InstancedStaticMesh|AddInstance (Variables|Default|GetHISM) (Math|Transform|MakeTransform (Math|Vector|MakeVector (Math|Conversions|ToFloat(Integer) _output_get_2) (Math|Conversions|ToFloat(Integer) _output_get_3) (Math|Conversions|ToFloat(Integer) _output_get_4)) (Math|Rotator|MakeRotator 0.0 0.0 0.0) (Math|Vector|MakeVector 1.0 1.0 1.0)))))))