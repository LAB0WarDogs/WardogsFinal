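; Shotgun skill component for BP_SecondChara, with an aim, fire or cancel flow and a recharge cooldown.
; Aiming locks the camera, lets the joystick drive the mouse cursor on Tick, and turns the character toward it through a self-recalling Delay loop.
; Firing box-overlaps at the melee point, box-traces to found actors for line of sight, and damages BPI_Damageable hits.
; Cleanup restores character state, starting the cooldown unless cancelled.
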(event Custom|ActivateFirstSkill
  (bind _secondchara (Variables|Default|GetSecondChara))
  (if (and (not (Variables|/Game/Blueprint/Character/CharacterMaster.CharacterMaster_C|GetIsUsingSkill (Variables|Default|GetSecondChara))) (Variables|Default|GetcooldownEnd))
    (Variables|/Game/Blueprint/Character/CharacterMaster.CharacterMaster_C|SetIsUsingSkill (Variables|Default|GetSecondChara) true)
    (Variables|/Game/Blueprint/Character/CharacterMaster.CharacterMaster_C|SetCanMoveWithUsingSkill _secondchara true)
    (Variables|/Game/Blueprint/Character/CharacterMaster.CharacterMaster_C|SetCantMoveCamera _secondchara true)
    (CallFunction|AimingFirstSkill)))

(event Custom|AimingFirstSkill
  (Components|Tick|SetComponentTickEnabled true)
  (Variables|Default|SetFacePlayer? true)
  (CallFunction|FacePlayer))

(event Custom|FacePlayer
  ;[0 0 1] Face Player
  (if (Variables|Default|GetFacePlayer?)
    (Transformation|SetActorRelativeRotation (Variables|Default|GetSecondChara) (Math|Rotator|MakeRotator 0.0 0.0 (.yaw (Math|Interpolation|RInterpTo (Transformation|GetActorRotation (Variables|Default|GetSecondChara)) (Math|Rotator|FindLookatRotation (Transformation|GetActorLocation (Variables|Default|GetSecondChara)) (.ImpactPoint (Collision|BreakHitResult (.HitResult (Game|Player|GetHitResultUnderCursorbyChannel (Game|GetPlayerController 0) "TraceTypeQuery1" true))))) (Utilities|Time|GetWorldDeltaSeconds) 2e+01))))
    (Utilities|FlowControl|Delay 0.001)
    (CallFunction|FacePlayer)))

(event Custom|UseFirstSkill
  (bind _secondchara (Variables|Default|GetSecondChara))
  (bind _meleeattack (Variables|/Game/Blueprint/Character/BP_SecondChara.BP_SecondChara_C|GetMeleeAttack _secondchara))
  (bind _returnvalue (Transformation|GetWorldLocation _meleeattack))
  (if (and (Variables|Default|GetcooldownEnd) (Variables|/Game/Blueprint/Character/CharacterMaster.CharacterMaster_C|GetIsUsingSkill (Variables|Default|GetSecondChara)))
    (Variables|Default|SetcooldownEnd false)
    (bind _outactors (Collision|BoxOverlapActors _returnvalue (Variables|Default|GetShotgunAOE) (Variables|Default|GetObject%20Types) 0 (Utilities|Array|MakeArray (Variables|Default|GetSecondChara)) :!class /Script/Engine.KismetSystemLibrary))
    (Rendering|Debug|DrawDebugBox _returnvalue (Variables|Default|GetShotgunAOE) "(R=1.000000,G=0.000000,B=0.000000,A=1.000000)" (Transformation|GetWorldRotation (Variables|/Script/Engine.Character|GetMesh _secondchara)) 1.0 0.0)
    (for _array_element _outactors
      (bind _outhit (Collision|BoxTraceByChannel (Transformation|GetWorldLocation (Variables|/Script/Engine.Actor|GetRootComponent (Variables|Default|GetSecondChara))) (Transformation|GetWorldLocation (Variables|/Script/Engine.Actor|GetRootComponent _array_element)) "10.000000,10.000000,10.000000" "0, 0, 0" "TraceTypeQuery1" false 0 "ForDuration"))
      (if (Utilities|DoesObjectImplementInterface (.HitActor (Collision|BreakHitResult _outhit)) "/Game/Blueprint/Interface/BPI_Damageable.BPI_Damageable_C")
        (Class|BPIDamageable|TakeDamage(Message) (.HitActor (Collision|BreakHitResult _outhit)) 5e+01))
      (Components|Tick|SetComponentTickEnabled false)
      (Variables|/Game/Blueprint/Character/CharacterMaster.CharacterMaster_C|SetIsUsingSkill (Variables|Default|GetSecondChara) false)
      (Variables|/Game/Blueprint/Character/CharacterMaster.CharacterMaster_C|SetCanMoveWithUsingSkill (Variables|Default|GetSecondChara) false)
      (Variables|/Game/Blueprint/Character/CharacterMaster.CharacterMaster_C|SetCantMoveCamera (Variables|Default|GetSecondChara) false)
      (Variables|Default|SetFacePlayer? false)
      (if (not (Variables|Default|GetIsCanceled))
        (Default|StartCooldown (Variables|Default|GetAs%20Character%20Master) (Variables|Default|GetRechargeShotgunCooldown))
        (Utilities|FlowControl|Delay (Variables|Default|GetRechargeShotgunCooldown))
        (Variables|Default|SetcooldownEnd true)
        (else
          (Variables|Default|SetIsCanceled false))))
    (Components|Tick|SetComponentTickEnabled false)
    (Variables|/Game/Blueprint/Character/CharacterMaster.CharacterMaster_C|SetIsUsingSkill (Variables|Default|GetSecondChara) false)
    (Variables|/Game/Blueprint/Character/CharacterMaster.CharacterMaster_C|SetCanMoveWithUsingSkill (Variables|Default|GetSecondChara) false)
    (Variables|/Game/Blueprint/Character/CharacterMaster.CharacterMaster_C|SetCantMoveCamera (Variables|Default|GetSecondChara) false)
    (Variables|Default|SetFacePlayer? false)
    (if (not (Variables|Default|GetIsCanceled))
      (Default|StartCooldown (Variables|Default|GetAs%20Character%20Master) (Variables|Default|GetRechargeShotgunCooldown))
      (Utilities|FlowControl|Delay (Variables|Default|GetRechargeShotgunCooldown))
      (Variables|Default|SetcooldownEnd true)
      (else
        (Variables|Default|SetIsCanceled false)))))

(event Custom|Cancelation
  (Variables|Default|SetIsCanceled true)
  (Components|Tick|SetComponentTickEnabled false)
  (Variables|/Game/Blueprint/Character/CharacterMaster.CharacterMaster_C|SetIsUsingSkill (Variables|Default|GetSecondChara) false)
  (Variables|/Game/Blueprint/Character/CharacterMaster.CharacterMaster_C|SetCanMoveWithUsingSkill (Variables|Default|GetSecondChara) false)
  (Variables|/Game/Blueprint/Character/CharacterMaster.CharacterMaster_C|SetCantMoveCamera (Variables|Default|GetSecondChara) false)
  (Variables|Default|SetFacePlayer? false)
  (if (not (Variables|Default|GetIsCanceled))
    (Default|StartCooldown (Variables|Default|GetAs%20Character%20Master) (Variables|Default|GetRechargeShotgunCooldown))
    (Utilities|FlowControl|Delay (Variables|Default|GetRechargeShotgunCooldown))
    (Variables|Default|SetcooldownEnd true)
    (else
      (Variables|Default|SetIsCanceled false))))

(event EventBeginPlay
  (bind _returnvalue (Actor|GetActorOfClass "/Game/Blueprint/Character/BP_SecondChara.BP_SecondChara_C"))
  (Variables|Default|SetSecondChara _returnvalue)
  (bind _ascharacter_master (CallFunction|GetPlayerCharacterMaster))
  (Variables|Default|SetAs%20Character%20Master _ascharacter_master))

(event EventTick
  (params (DeltaSeconds :type Float%20%28single-precision%29))
  (bind _returnvalue (Game|GetPlayerController 0))
  (bind (_sizex _sizey) (HUD|GetViewportSize _returnvalue))
  (bind _asmy_player_controller (CallFunction|GetPlayerController))
  (Class|PlayerController|SetMouseLocation (Game|GetPlayerController 0) (Math|Integer|Clamp(Integer) (Math|Float|Truncate (+ (.LocationX (Game|Player|GetMousePosition _asmy_player_controller)) (* (Variables|/Game/Blueprint/Character/MyPlayerController.MyPlayerController_C|GetJoystickX _asmy_player_controller) 2e+01))) 0 _sizex) (Math|Integer|Clamp(Integer) (Math|Float|Truncate (+ (.LocationY (Game|Player|GetMousePosition _asmy_player_controller)) (* (Variables|/Game/Blueprint/Character/MyPlayerController.MyPlayerController_C|GetJoystickY _asmy_player_controller) 2e+01))) 0 _sizey)))