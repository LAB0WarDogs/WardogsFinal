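; BP_DroneSkill is a skill component that lets the player deploy and pilot a drone as a second skill.
; Activation, allowed only while the player has the drone, spawns BP_Drone at the character's DroneRoot, stops the character's movement and hands player control to the drone.
; Cancelation possesses the character again and clears the active flag, without destroying the drone or restoring its availability here.
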(event Custom|ActivateSecondSkill
  (bind _as_bp_first_chara (Variables|Default|GetAs%20BP%20First%20Chara))
  (bind _droneroot (Variables|/Game/Blueprint/Character/BP_FirstChara.BP_FirstChara_C|GetDroneRoot _as_bp_first_chara))
  (bind _returnvalue (Transformation|GetWorldLocation _droneroot))
  (if (Variables|Default|GetPlayerHasDrone?)
    (Utilities|FlowControl|Sequence
      (:then_0
        (Variables|Default|SetPlayerHasDrone? false)
        (Variables|Default|SetDroneIsActive? true)
        (bind _returnvalue_2 (Game|SpawnActorfromClass "/Game/Blueprint/Actors/Drone/BP_Drone.BP_Drone_C" (Math|Transform|MakeTransform (Math|Vector|MakeVector (.x _returnvalue) (.y _returnvalue) (.z _returnvalue)) "0, 0, 0" "1,1,1") "AdjustIfPossibleButAlwaysSpawn" 0 0))
        (Variables|Default|SetBP_DroneRef _returnvalue_2)
        (Components|Movement|StopMovementImmediately (Variables|/Script/Engine.Character|GetCharacterMovement (Variables|Default|GetAs%20BP%20First%20Chara))))
      (:then_1
        (Class|Pawn|DetachfromControllerPendingDestroy (Variables|Default|GetBP_DroneRef))
        (Pawn|Possess (Game|GetPlayerController 0) (Variables|Default|GetBP_DroneRef))
        (Pawn|SpawnDefaultController (Variables|Default|GetBP_DroneRef))))
    (else
      (Development|PrintString "Player doesn't have the drone"))))

(event Custom|Cancelation
  (Class|Pawn|DetachfromControllerPendingDestroy (Variables|Default|GetAs%20BP%20First%20Chara))
  (Pawn|Possess (Game|GetPlayerController 0) (Variables|Default|GetAs%20BP%20First%20Chara))
  (Pawn|SpawnDefaultController (Variables|Default|GetAs%20BP%20First%20Chara))
  (Variables|Default|SetDroneIsActive? false))

(event EventBeginPlay
  (bind _asbp_first_chara (Utilities|Casting|CastToBP_FirstChara (Game|GetPlayerCharacter 0)))
  (Variables|Default|SetAs%20BP%20First%20Chara _asbp_first_chara))