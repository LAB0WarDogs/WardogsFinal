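; Flair skill component for BP_FirstChara that reveals nearby AI to the player.
; Activation plays a sound and runs a debug-drawn sphere overlap just ahead of the character.
; Highlightable BP_AI_Master hits show their Niagara trace and custom-depth outline, then call their hide routine.
; The cooldown and use-flag reset run inside the hit loop, so an empty overlap leaves the character flagged as using a skill.
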(event Custom|ActivateSecondSkill
  (bind _firstchararef (Variables|Default|GetFirstCharaRef))
  (if (and (not (Variables|/Game/Blueprint/Character/CharacterMaster.CharacterMaster_C|GetIsUsingSkill (Variables|Default|GetFirstCharaRef))) (Variables|Default|GetCooldownOver?))
    (Variables|/Game/Blueprint/Character/CharacterMaster.CharacterMaster_C|SetIsUsingSkill _firstchararef true)
    (Variables|/Game/Blueprint/Character/CharacterMaster.CharacterMaster_C|SetCanMoveWithUsingSkill _firstchararef true)
    (CallFunction|UseSecondSkill)))

(event Custom|UseSecondSkill
  (bind _firstchararef (Variables|Default|GetFirstCharaRef))
  (bind _firstchararef_2 (Variables|Default|GetFirstCharaRef))
  (bind _returnvalue (Transformation|GetActorLocation _firstchararef_2))
  (bind _returnvalue_2 (Transformation|GetActorForwardVector _firstchararef_2))
  (bind _returnvalue_3 (* _returnvalue_2 "50.000000,50.000000,0.000000"))
  (bind _returnvalue_4 (+ _returnvalue _returnvalue_3))
  (if (Variables|/Game/Blueprint/Character/CharacterMaster.CharacterMaster_C|GetIsUsingSkill (Variables|Default|GetFirstCharaRef))
    (Audio|PlaySoundatLocation "/Game/Sound/Chien/SQ_Flair_Cue.SQ_Flair_Cue" (Transformation|GetActorLocation (Variables|Default|GetFirstCharaRef)) "0, 0, 0" 1.0 1.0 0.0 0 0 0 0)
    (Rendering|Debug|DrawDebugSphere _returnvalue_4 (Variables|Default|GetRadius) 12 "(R=1.000000,G=0.000000,B=0.000000,A=1.000000)" 2.0)
    (bind _outactors (Collision|SphereOverlapActors _returnvalue_4 (Variables|Default|GetRadius) (Variables|Default|GetObject%20Types) 0))
    (for _array_element _outactors
      (if (Utilities|DoesObjectImplementInterface _array_element "/Game/Blueprint/Interface/BPI_HighlightedActor.BPI_HighlightedActor_C")
        (Development|PrintString (Utilities|GetDisplayName _array_element))
        (bind _asbp_ai_master (Utilities|Casting|CastToBP_AI_Master _array_element))
        (Development|SetHiddeninGame (Variables|/Game/Blueprint/AI/AI_Puces/AiCharacter/BP_AI_PucesSentinel.BP_AI_PucesSentinel_C|GetNS_TempoPuceTrace _asbp_ai_master) false false)
        (Rendering|SetRenderCustomDepth (Variables|/Script/Engine.Character|GetMesh _asbp_ai_master) true)
        (Default|HIdeOutlineandVFX _asbp_ai_master))
      (Default|StartCooldown (Variables|Default|GetFirstCharaRef) (Variables|Default|GetCoolDown))
      (Utilities|FlowControl|Delay (Variables|Default|GetCoolDown))
      (Variables|Default|SetCooldownOver? true)
      (Variables|/Game/Blueprint/Character/CharacterMaster.CharacterMaster_C|SetIsUsingSkill _firstchararef false)
      (Variables|/Game/Blueprint/Character/CharacterMaster.CharacterMaster_C|SetCanMoveWithUsingSkill _firstchararef false))))

(event EventTick
  (params (DeltaSeconds :type Float%20%28single-precision%29)))

(event EventBeginPlay
  (bind _returnvalue (Actor|GetActorOfClass "/Game/Blueprint/Character/BP_FirstChara.BP_FirstChara_C"))
  (Variables|Default|SetFirstCharaRef _returnvalue))