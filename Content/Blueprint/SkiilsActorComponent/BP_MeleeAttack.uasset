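; Melee skill component for BP_SecondChara that damages enemies in a box around its attack point, using Shotgun-named cooldown and area variables.
; A box trace to each overlapped actor applies fixed damage through BPI_Damageable, sparing CharacterMaster hits, with debug shapes drawn.
; Each trace and loop completion feeds a shared reset that clears skill flags, disables tick and starts the cooldown.
; Cancelation uses that reset but skips the cooldown.
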(event Custom|UseFirstSkill
  (bind _secondchara (Variables|Default|GetSecondChara))
  (bind _meleeattack (Variables|/Game/Blueprint/Character/BP_SecondChara.BP_SecondChara_C|GetMeleeAttack _secondchara))
  (bind _returnvalue (Transformation|GetWorldLocation _meleeattack))
  (if (Variables|Default|GetcooldownEnd)
    (Variables|/Game/Blueprint/Character/CharacterMaster.CharacterMaster_C|SetIsUsingSkill (Variables|Default|GetSecondChara) true)
    (Variables|Default|SetcooldownEnd false)
    (Variables|/Game/Blueprint/Character/CharacterMaster.CharacterMaster_C|SetIsAttackingChowChow (Variables|Default|GetSecondChara) true)
    (bind _outactors (Collision|BoxOverlapActors _returnvalue (Variables|Default|GetShotgunAOE) (Variables|Default|GetObject%20Types) 0 (Utilities|Array|MakeArray (Variables|Default|GetSecondChara)) :!class /Script/Engine.KismetSystemLibrary))
    (Rendering|Debug|DrawDebugBox _returnvalue (Variables|Default|GetShotgunAOE) "(R=1.000000,G=0.000000,B=0.000000,A=1.000000)" (Transformation|GetWorldRotation (Variables|/Script/Engine.Character|GetMesh _secondchara)) 1.0 0.0)
    (for _array_element _outactors
      (bind _outhit (Collision|BoxTraceByChannel (Transformation|GetWorldLocation (Variables|/Script/Engine.Actor|GetRootComponent (Variables|Default|GetSecondChara))) (Transformation|GetWorldLocation (Variables|/Script/Engine.Actor|GetRootComponent _array_element)) "10.000000,10.000000,10.000000" "0, 0, 0" "TraceTypeQuery6" false (Utilities|Array|MakeArray (Variables|Default|GetAs%20Character%20Master)) "ForDuration"))
      (Utilities|Casting|CastToCharacterMaster (.HitActor (Collision|BreakHitResult _outhit))
        (:then
          _)
        (:CastFailed
          (if (Utilities|DoesObjectImplementInterface (.HitActor (Collision|BreakHitResult _outhit)) "/Game/Blueprint/Interface/BPI_Damageable.BPI_Damageable_C")
            (Class|BPIDamageable|TakeDamage(Message) (.HitActor (Collision|BreakHitResult _outhit)) 1e+02))))
      (Components|Tick|SetComponentTickEnabled false)
      (Variables|/Game/Blueprint/Character/CharacterMaster.CharacterMaster_C|SetIsUsingSkill (Variables|Default|GetSecondChara) false)
      (Variables|/Game/Blueprint/Character/CharacterMaster.CharacterMaster_C|SetCanMoveWithUsingSkill (Variables|Default|GetSecondChara) false)
      (Variables|/Game/Blueprint/Character/CharacterMaster.CharacterMaster_C|SetCantMoveCamera (Variables|Default|GetSecondChara) false)
      (Variables|Default|SetFacePlayer? false)
      (Utilities|FlowControl|Sequence
        (:then_0
          (if (not (Variables|Default|GetIsCanceled))
            (Default|StartCooldown (Variables|Default|GetAs%20Character%20Master) (Variables|Default|GetRechargeShotgunCooldown))
            (Utilities|FlowControl|Delay (Variables|Default|GetRechargeShotgunCooldown))
            (Variables|Default|SetcooldownEnd true)
            (else
              (Variables|Default|SetIsCanceled false))))
        (:then_1
          (Utilities|FlowControl|Delay 0.35)
          (Variables|/Game/Blueprint/Character/CharacterMaster.CharacterMaster_C|SetIsAttackingChowChow (Variables|Default|GetSecondChara) false))))
    (Components|Tick|SetComponentTickEnabled false)
    (Variables|/Game/Blueprint/Character/CharacterMaster.CharacterMaster_C|SetIsUsingSkill (Variables|Default|GetSecondChara) false)
    (Variables|/Game/Blueprint/Character/CharacterMaster.CharacterMaster_C|SetCanMoveWithUsingSkill (Variables|Default|GetSecondChara) false)
    (Variables|/Game/Blueprint/Character/CharacterMaster.CharacterMaster_C|SetCantMoveCamera (Variables|Default|GetSecondChara) false)
    (Variables|Default|SetFacePlayer? false)
    (Utilities|FlowControl|Sequence
      (:then_0
        (if (not (Variables|Default|GetIsCanceled))
          (Default|StartCooldown (Variables|Default|GetAs%20Character%20Master) (Variables|Default|GetRechargeShotgunCooldown))
          (Utilities|FlowControl|Delay (Variables|Default|GetRechargeShotgunCooldown))
          (Variables|Default|SetcooldownEnd true)
          (else
            (Variables|Default|SetIsCanceled false))))
      (:then_1
        (Utilities|FlowControl|Delay 0.35)
        (Variables|/Game/Blueprint/Character/CharacterMaster.CharacterMaster_C|SetIsAttackingChowChow (Variables|Default|GetSecondChara) false)))))

(event Custom|Cancelation
  (Variables|Default|SetIsCanceled true)
  (Components|Tick|SetComponentTickEnabled false)
  (Variables|/Game/Blueprint/Character/CharacterMaster.CharacterMaster_C|SetIsUsingSkill (Variables|Default|GetSecondChara) false)
  (Variables|/Game/Blueprint/Character/CharacterMaster.CharacterMaster_C|SetCanMoveWithUsingSkill (Variables|Default|GetSecondChara) false)
  (Variables|/Game/Blueprint/Character/CharacterMaster.CharacterMaster_C|SetCantMoveCamera (Variables|Default|GetSecondChara) false)
  (Variables|Default|SetFacePlayer? false)
  (Utilities|FlowControl|Sequence
    (:then_0
      (if (not (Variables|Default|GetIsCanceled))
        (Default|StartCooldown (Variables|Default|GetAs%20Character%20Master) (Variables|Default|GetRechargeShotgunCooldown))
        (Utilities|FlowControl|Delay (Variables|Default|GetRechargeShotgunCooldown))
        (Variables|Default|SetcooldownEnd true)
        (else
          (Variables|Default|SetIsCanceled false))))
    (:then_1
      (Utilities|FlowControl|Delay 0.35)
      (Variables|/Game/Blueprint/Character/CharacterMaster.CharacterMaster_C|SetIsAttackingChowChow (Variables|Default|GetSecondChara) false))))

(event EventBeginPlay
  (bind _returnvalue (Actor|GetActorOfClass "/Game/Blueprint/Character/BP_SecondChara.BP_SecondChara_C"))
  (Variables|Default|SetSecondChara _returnvalue)
  (bind _ascharacter_master (CallFunction|GetPlayerCharacterMaster))
  (Variables|Default|SetAs%20Character%20Master _ascharacter_master))