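; IEM skill component for the third-person character that stuns AI enemies in front of the player.
; ActivateSecondSkill checks the character's skill-in-use flag and cooldown, then runs a debug-drawn sphere overlap ahead of the character.
; Damageable BP_AI_Master actors get stunned through their AI controller.
; Each overlapped actor, hit or not, leads into the cooldown and flag reset, so an empty overlap leaves the skill flagged in use.
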(event Custom|ActivateSecondSkill
  (if (and (not (Variables|/Game/Blueprint/Character/CharacterMaster.CharacterMaster_C|GetIsUsingSkill (Variables|Default|GetThirdCharaRef))) (Variables|Default|GetCooldownOver?))
    (Variables|/Game/Blueprint/Character/CharacterMaster.CharacterMaster_C|SetIsUsingSkill (Variables|Default|GetThirdCharaRef) true)
    (CallFunction|UseSecondSkill)))

(event Custom|UseSecondSkill
  (bind _cooldownbeforeactifagain (Variables|Default|GetCooldownBeforeActifAgain))
  (bind _thirdchararef (Variables|Default|GetThirdCharaRef))
  (bind _returnvalue (Transformation|GetActorLocation _thirdchararef))
  (bind _returnvalue_2 (Transformation|GetActorForwardVector _thirdchararef))
  (bind _returnvalue_3 (* _returnvalue_2 "50.000000,50.000000,0.000000"))
  (bind _returnvalue_4 (+ _returnvalue _returnvalue_3))
  (if (Variables|/Game/Blueprint/Character/CharacterMaster.CharacterMaster_C|GetIsUsingSkill (Variables|Default|GetThirdCharaRef))
    (Rendering|Debug|DrawDebugSphere _returnvalue_4 (Variables|Default|GetRadius) 12 "(R=1.000000,G=0.000000,B=0.000000,A=1.000000)" 2.0)
    (bind _outactors (Collision|SphereOverlapActors _returnvalue_4 (Variables|Default|GetRadius) (Variables|Default|GetObject%20Types) 0))
    (for _array_element _outactors
      (if (Utilities|DoesObjectImplementInterface _array_element "/Game/Blueprint/Interface/BPI_Damageable.BPI_Damageable_C")
        (bind _asbp_ai_master (Utilities|Casting|CastToBP_AI_Master _array_element)
          (:then
            (bind _asbp_ai_controller_master (Utilities|Casting|CastToBP_AiControllerMaster (AI|GetAIController _asbp_ai_master)))
            (Default|Stunned _asbp_ai_controller_master 5.0)
            (Variables|Default|SetCooldownOver? false)
            (Variables|/Game/Blueprint/Character/CharacterMaster.CharacterMaster_C|SetIsUsingSkill (Variables|Default|GetThirdCharaRef) false)
            (Default|StartCooldown (Variables|Default|GetThirdCharaRef) _cooldownbeforeactifagain)
            (Utilities|FlowControl|Delay _cooldownbeforeactifagain)
            (Variables|Default|SetCooldownOver? true))
          (:CastFailed
            (CallFunction|NoHit :!label _label)))
        (else
          (goto _label))))))

(event Custom|NoHit
  (bind _cooldownbeforeactifagain (Variables|Default|GetCooldownBeforeActifAgain))
  (Variables|Default|SetCooldownOver? false)
  (Variables|/Game/Blueprint/Character/CharacterMaster.CharacterMaster_C|SetIsUsingSkill (Variables|Default|GetThirdCharaRef) false)
  (Default|StartCooldown (Variables|Default|GetThirdCharaRef) _cooldownbeforeactifagain)
  (Utilities|FlowControl|Delay _cooldownbeforeactifagain)
  (Variables|Default|SetCooldownOver? true))

(event EventBeginPlay
  (bind _returnvalue (Actor|GetActorOfClass "/Game/Blueprint/Character/BP_ThirdChara.BP_ThirdChara_C"))
  (Variables|Default|SetThirdCharaRef _returnvalue))