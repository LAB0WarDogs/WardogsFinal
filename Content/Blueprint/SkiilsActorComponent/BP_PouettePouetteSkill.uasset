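; Skill component for BP_SecondChara that aims and throws a "PouettePouette" grenade, consuming a battery and starting a cooldown.
; Aiming halves time dilation, turns the character toward the cursor, which also accepts joystick input, and colors a target marker by range.
; A delay-driven loop places pooled point actors along the predicted arc.
; Launch direction runs from character through GrenadeRef, with speed equal to cursor distance.
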(event Custom|ActivatSegondSkill
  (bind _secondchararef (Variables|Default|GetSecondCharaRef))
  (if (and (not (Variables|/Game/Blueprint/Character/CharacterMaster.CharacterMaster_C|GetIsUsingSkill (Variables|Default|GetSecondCharaRef))) (Variables|Default|GetCoolDownIsOver))
    (Variables|/Game/Blueprint/Character/CharacterMaster.CharacterMaster_C|SetIsUsingSkill (Variables|Default|GetSecondCharaRef) true)
    (Variables|/Game/Blueprint/Character/CharacterMaster.CharacterMaster_C|SetCanMoveWithUsingSkill _secondchararef true)
    (Variables|/Game/Blueprint/Character/CharacterMaster.CharacterMaster_C|SetCantMoveCamera _secondchararef true)
    (Components|Tick|SetComponentTickEnabled true)
    (CallFunction|AimingThirdSkill)))

(event Custom|AimingThirdSkill
  (bind _returnvalue (Game|GetPlayerController 0))
  (bind (_sizex _sizey) (HUD|GetViewportSize _returnvalue))
  (Utilities|FlowControl|Sequence
    (:then_0
      (Variables|Default|SetFacePlayer? true)
      (CallFunction|FacePlayer)
      (Rendering|SetVisibility (Variables|Default|GetGrenade%20Target) true true)
      (Transformation|DetachFromComponent (Variables|Default|GetGrenade%20Target) "KeepWorld" "KeepWorld" "KeepWorld" true)
      (Class|PlayerController|SetMouseLocation (Game|GetPlayerController 0) (/ _sizex 2) (/ _sizey 2))
      (Utilities|Time|SetGlobalTimeDilation 0.5))
    (:then_1
      (Variables|Default|SetIsAiming? true)
      (CallFunction|Predict))
    (:then_2
      (CallFunction|GetPosition))
    (:then_3
      (Variables|/Game/Blueprint/Character/CharacterMaster.CharacterMaster_C|SetIsArmingGrenade (Variables|Default|GetSecondCharaRef) true))))

(event Custom|FacePlayer
  (if (Variables|Default|GetFacePlayer?)
    (Transformation|SetActorRelativeRotation (Variables|Default|GetSecondCharaRef) (Math|Rotator|MakeRotator 0.0 0.0 (.yaw (Math|Interpolation|RInterpTo (Transformation|GetActorRotation (Variables|Default|GetSecondCharaRef)) (Math|Rotator|FindLookatRotation (Transformation|GetActorLocation (Variables|Default|GetSecondCharaRef)) (.ImpactPoint (Collision|BreakHitResult (.HitResult (Game|Player|GetHitResultUnderCursorbyChannel (Game|GetPlayerController 0) "TraceTypeQuery1" true))))) (Utilities|Time|GetWorldDeltaSeconds) 2e+01))))
    (Utilities|FlowControl|Delay 0.001)
    (CallFunction|FacePlayer)))

(event Custom|UsingSegondSkill
  (bind _aimpoints (Variables|Default|GetAimPoints))
  (bind _secondchararef (Variables|Default|GetSecondCharaRef))
  (bind _cooldownduration (Variables|Default|GetCoolDownDuration))
  (if (and (Variables|/Game/Blueprint/Character/CharacterMaster.CharacterMaster_C|GetIsUsingSkill (Variables|Default|GetSecondCharaRef)) (Variables|Default|GetIsInRange))
    (Variables|Default|SetCoolDownIsOver false)
    (Variables|/Game/Blueprint/Character/CharacterMaster.CharacterMaster_C|SetIsArmingGrenade _secondchararef false)
    (Variables|/Game/Blueprint/Character/CharacterMaster.CharacterMaster_C|SetIsLaunchingGrenade _secondchararef true)
    (Utilities|FlowControl|Delay 0.2)
    (bind _returnvalue (Game|SpawnActorfromClass "/Game/Blueprint/Actors/Grenade/BP_PouettePouetteGre.BP_PouettePouetteGre_C" (Math|Transform|MakeTransform (Transformation|GetWorldLocation (Variables|Default|GetGrenade%20Ref)) (Transformation|GetActorRotation (Variables|Default|GetSecondCharaRef)) "1.000000,1.000000,1.000000") "Undefined" 0 0))
    (Physics|SetPhysicsLinearVelocity (Variables|/Game/Blueprint/Actors/Grenade/BP_PouettePouetteGre.BP_PouettePouetteGre_C|GetSphere _returnvalue) (* (Math|Vector|GetUnitDirection(Vector) (Transformation|GetActorLocation (Variables|Default|GetSecondCharaRef)) (Transformation|GetActorLocation _returnvalue)) (CallFunction|GetSpeedBaseDistancefromPlayer)) false "None")
    (Default|CallUseBatteryfromInventory (Variables|Default|GetAs%20Character%20Master))
    (Variables|/Game/Blueprint/Character/CharacterMaster.CharacterMaster_C|SetIsUsingSkill (Variables|Default|GetSecondCharaRef) false)
    (Variables|/Game/Blueprint/Character/CharacterMaster.CharacterMaster_C|SetCanMoveWithUsingSkill (Variables|Default|GetSecondCharaRef) false)
    (Variables|/Game/Blueprint/Character/CharacterMaster.CharacterMaster_C|SetCantMoveCamera (Variables|Default|GetSecondCharaRef) false)
    (Variables|Default|SetIsAiming? false)
    (Variables|/Game/Blueprint/Character/CharacterMaster.CharacterMaster_C|SetIsArmingGrenade (Variables|Default|GetSecondCharaRef) false)
    (Utilities|FlowControl|Sequence
      (:then_0
        (Variables|Default|SetFacePlayer? false)
        (Rendering|SetVisibility (Variables|Default|GetGrenade%20Target) false true)
        (Utilities|Time|SetGlobalTimeDilation 1.0)
        (if (not (Variables|Default|GetIsCanceled))
          (Default|StartCooldown (Variables|Default|GetAs%20Character%20Master) _cooldownduration)
          (Utilities|FlowControl|Delay _cooldownduration))
        (Components|Tick|SetComponentTickEnabled false)
        (Variables|Default|SetCoolDownIsOver true)
        (Variables|Default|SetIsCanceled false))
      (:then_1
        ;[1 1 1] Aim Visibility
        (for _array_element _aimpoints
          (Actor|DestroyActor _array_element))
        (Utilities|Array|Clear _aimpoints)
        (Utilities|FlowControl|Delay 0.2)
        (Variables|/Game/Blueprint/Character/CharacterMaster.CharacterMaster_C|SetIsLaunchingGrenade (Variables|Default|GetSecondCharaRef) false)))))

(event Custom|get%20position
  (bind _secondchararef (Variables|Default|GetSecondCharaRef))
  (bind _grenade_target (Variables|Default|GetGrenade%20Target))
  (bind _returnvalue (Transformation|GetWorldLocation _grenade_target))
  (bind _rootcomponent (Variables|/Script/Engine.Actor|GetRootComponent _secondchararef))
  (bind _returnvalue_2 (Transformation|GetWorldLocation _rootcomponent))
  (if (and (> (Math|Float|Sqrt (+ (Math|Float|Square (- (.x _returnvalue) (.x _returnvalue_2))) (Math|Float|Square (- (.y _returnvalue) (.y _returnvalue_2))))) (Variables|Default|GetThrowingMaxDistance)) (Variables|Default|GetIsAiming?))
    (Rendering|Material|SetMaterial (Variables|Default|GetGrenade%20Target) 0 "/Engine/EngineDebugMaterials/VertexColorViewMode_RedOnly.VertexColorViewMode_RedOnly")
    (Variables|Default|SetIsInRange false)
    (else
      (Rendering|Material|SetMaterial (Variables|Default|GetGrenade%20Target) 0 "/Engine/EngineDebugMaterials/VertexColorViewMode_GreenOnly.VertexColorViewMode_GreenOnly")
      (Variables|Default|SetIsInRange true)))
  (Utilities|FlowControl|Delay 0.2)
  (CallFunction|GetPosition))

(event Custom|Cancelation
  (bind _aimpoints (Variables|Default|GetAimPoints))
  (bind _cooldownduration (Variables|Default|GetCoolDownDuration))
  (Variables|Default|SetIsCanceled true)
  (Variables|/Game/Blueprint/Character/CharacterMaster.CharacterMaster_C|SetIsUsingSkill (Variables|Default|GetSecondCharaRef) false)
  (Variables|/Game/Blueprint/Character/CharacterMaster.CharacterMaster_C|SetCanMoveWithUsingSkill (Variables|Default|GetSecondCharaRef) false)
  (Variables|/Game/Blueprint/Character/CharacterMaster.CharacterMaster_C|SetCantMoveCamera (Variables|Default|GetSecondCharaRef) false)
  (Variables|Default|SetIsAiming? false)
  (Variables|/Game/Blueprint/Character/CharacterMaster.CharacterMaster_C|SetIsArmingGrenade (Variables|Default|GetSecondCharaRef) false)
  (Utilities|FlowControl|Sequence
    (:then_0
      (Variables|Default|SetFacePlayer? false)
      (Rendering|SetVisibility (Variables|Default|GetGrenade%20Target) false true)
      (Utilities|Time|SetGlobalTimeDilation 1.0)
      (if (not (Variables|Default|GetIsCanceled))
        (Default|StartCooldown (Variables|Default|GetAs%20Character%20Master) _cooldownduration)
        (Utilities|FlowControl|Delay _cooldownduration))
      (Components|Tick|SetComponentTickEnabled false)
      (Variables|Default|SetCoolDownIsOver true)
      (Variables|Default|SetIsCanceled false))
    (:then_1
      ;[1 1 1] Aim Visibility
      (for _array_element _aimpoints
        (Actor|DestroyActor _array_element))
      (Utilities|Array|Clear _aimpoints)
      (Utilities|FlowControl|Delay 0.2)
      (Variables|/Game/Blueprint/Character/CharacterMaster.CharacterMaster_C|SetIsLaunchingGrenade (Variables|Default|GetSecondCharaRef) false))))

(event Custom|predict
  (bind _aimpoints (Variables|Default|GetAimPoints))
  (bind _grenade_ref (Variables|Default|GetGrenade%20Ref))
  (bind _returnvalue (Transformation|GetWorldLocation _grenade_ref))
  ;[1 1 1] Prediction
  (if (Variables|Default|GetIsAiming?)
    (bind _outpathpositions (Class|GameplayStatics|BlueprintPredictProjectilePathbyObjectType _returnvalue (* (Math|Vector|GetUnitDirection(Vector) (Transformation|GetActorLocation (Variables|Default|GetSecondCharaRef)) _returnvalue) (CallFunction|GetSpeedBaseDistancefromPlayer)) true 2e+01 (Utilities|Array|MakeArray "ObjectTypeQuery1") false 0 "None" 0.0 1e+01))
    (Utilities|FlowControl|Sequence
      (:then_0
        (for (_array_element _array_index) _outpathpositions
          (if (> (Math|Conversions|ToFloat(Integer) _array_index) (Math|Conversions|ToFloat(Integer) (Utilities|Array|LastIndex _aimpoints)))
            (bind _returnvalue_2 (Game|SpawnActorfromClass "/Game/Blueprint/SkiilsActorComponent/AimPoints.AimPoints_C" (Math|Transform|MakeTransform _array_element "0, 0, 0" "0.100000,0.100000,0.100000") "Undefined" 0 0))
            (Utilities|Array|SetArrayElem _aimpoints _array_index _returnvalue_2 true))))
      (:then_1
        (for (_array_element_2 _array_index_2) _aimpoints
          (if (>= (Utilities|Array|LastIndex _outpathpositions) _array_index_2)
            (Transformation|SetWorldLocation (Variables|/Script/Engine.Actor|GetRootComponent _array_element_2) (Utilities|Array|Get(acopy) _outpathpositions _array_index_2) false true)
            (else
              (Transformation|SetWorldLocation (Variables|/Script/Engine.Actor|GetRootComponent _array_element_2) "10000.000000, 0, 0" false true)))))
      (:then_2
        (Utilities|FlowControl|Delay 0.01)
        (CallFunction|Predict)))))

(event EventTick
  (params (DeltaSeconds :type Float%20%28single-precision%29))
  (bind _returnvalue (Game|GetPlayerController 0))
  (bind (_sizex _sizey) (HUD|GetViewportSize _returnvalue))
  (bind _asmy_player_controller (CallFunction|GetPlayerController))
  (Class|PlayerController|SetMouseLocation (Game|GetPlayerController 0) (Math|Integer|Clamp(Integer) (Math|Float|Truncate (+ (.LocationX (Game|Player|GetMousePosition _asmy_player_controller)) (* (Variables|/Game/Blueprint/Character/MyPlayerController.MyPlayerController_C|GetJoystickX _asmy_player_controller) 2e+01))) 0 _sizex) (Math|Integer|Clamp(Integer) (Math|Float|Truncate (+ (.LocationY (Game|Player|GetMousePosition _asmy_player_controller)) (* (Variables|/Game/Blueprint/Character/MyPlayerController.MyPlayerController_C|GetJoystickY _asmy_player_controller) 2e+01))) 0 _sizey))
  (Components|MoveComponentTo (Variables|Default|GetGrenade%20Target) (.ImpactPoint (Collision|BreakHitResult (.HitResult (Game|Player|GetHitResultUnderCursorbyChannel (Game|GetPlayerController 0) "TraceTypeQuery6" true)))) "-90.000000,0.000000, 0" false false 0.1 false))

(event EventBeginPlay
  (bind _returnvalue (Actor|GetActorOfClass "/Game/Blueprint/Character/BP_SecondChara.BP_SecondChara_C"))
  (bind _output_get (Variables|Default|SetSecondCharaRef _returnvalue))
  (Variables|Default|SetGrenade%20Target (Variables|/Game/Blueprint/Character/BP_SecondChara.BP_SecondChara_C|GetGrenadeTarget _returnvalue))
  (Variables|Default|SetGrenade%20Ref (Variables|/Game/Blueprint/Character/BP_SecondChara.BP_SecondChara_C|GetGrenadeRef _returnvalue))
  (bind _ascharacter_master (CallFunction|GetPlayerCharacterMaster))
  (Variables|Default|SetAs%20Character%20Master _ascharacter_master)
  (Variables|Default|SetOriginal%20World%20Scale (Transformation|GetWorldScale (Variables|/Game/Blueprint/Character/CharacterMaster.CharacterMaster_C|GetNoiseArea _output_get))))

(fn AlwaysFacePlayer)

(fn GetSpeedBaseDistancefromPlayer
  (return (Math|Vector|Distance(Vector) (.ImpactPoint (Collision|BreakHitResult (.HitResult (Game|Player|GetHitResultUnderCursorbyChannel (Game|GetPlayerController 0) "TraceTypeQuery1" true)))) (Transformation|GetActorLocation (Variables|Default|GetSecondCharaRef)))))