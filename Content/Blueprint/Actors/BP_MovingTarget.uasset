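; BP_MovingTarget is an actor that shuttles its BPTarget back and forth between the Pose2 and Pose1 world positions, starting on BeginPlay.
; A timeline lerps the target's location without sweeping, with play rate scaled by the Time variable.
; When the timeline finishes, it pauses for a tenth of Time, then a toggled flag chooses between replaying from the start and reversing.
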(event Custom|Move
  (Components|Timeline|SetPlayRate (Variables|Default|GetTimeline_0) (/ 1.0 (Variables|Default|GetTime)))
  (bind _time (Timeline|Timeline_0 PlayFromStart)
    (:Update
      (Transformation|SetWorldLocation (Variables|Default|GetBP_Target) (Math|Vector|Lerp(Vector) (Transformation|GetWorldLocation (Variables|Default|GetPose_2)) (Transformation|GetWorldLocation (Variables|Default|GetPose_1)) _time) false false))
    (:Finished
      (Utilities|FlowControl|Delay (/ (Variables|Default|GetTime) 1e+01))
      (if (Variables|Default|GetPose1)
        (Variables|Default|SetPose1 false)
        (CallFunction|Move)
        (else
          (Variables|Default|SetPose1 true)
          (Timeline|Timeline_0 Reverse))))))

(event EventBeginPlay
  (CallFunction|Move))

(fn ConstructionScript)