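; Checkpoint actor that records a respawn position the first time a CharacterMaster overlaps its Box.
; A DoOnce writes the checkpoint's own location and rotation, with unit scale, into PlayerPos on the GameModeWardogs save object and saves it to slot "save1".
; When that slot does not exist, it only fills a new BP_SaveGame object, which is neither stored nor written to disk.
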(event OnComponentBeginOverlap(Box)
  (params (OverlappedComponent :type Primitive%20Component%20Object%20Reference) (OtherActor :type Actor%20Object%20Reference) (OtherComp :type Primitive%20Component%20Object%20Reference) (OtherBodyIndex :type Integer) (bFromSweep :type Boolean) (SweepResult :type Hit%20Result%20Structure%20%28by%20ref%29))
  (bind _self self)
  (bind _returnvalue (Transformation|GetActorTransform _self))
  (bind _returnvalue_2 (Transformation|GetActorTransform _self))
  (Utilities|Casting|CastToCharacterMaster OtherActor)
  (Utilities|FlowControl|DoOnce false
    (:Completed
      (bind _returnvalue_3 (SaveGame|DoesSaveGameExist "save1"))
      (if _returnvalue_3
        (bind _asgame_mode_wardogs (Utilities|Casting|CastToGameModeWardogs (Game|GetGameMode)))
        (Variables|/Game/Blueprint/BP_SaveGame.BP_SaveGame_C|SetPlayerPos (Variables|/Game/Blueprint/GameMode/GameModeWardogs.GameModeWardogs_C|GetAs%20BP%20Save%20Game _asgame_mode_wardogs) (Math|Transform|MakeTransform (.location _returnvalue_2) (.rotation _returnvalue_2) "1.000000,1.000000,1.000000"))
        (SaveGame|SaveGametoSlot (Variables|/Game/Blueprint/GameMode/GameModeWardogs.GameModeWardogs_C|GetAs%20BP%20Save%20Game _asgame_mode_wardogs) "save1")
        (else
          (bind _returnvalue_4 (SaveGame|CreateSaveGameObject "/Game/Blueprint/BP_SaveGame.BP_SaveGame_C"))
          (Variables|/Game/Blueprint/BP_SaveGame.BP_SaveGame_C|SetPlayerPos _returnvalue_4 (Math|Transform|MakeTransform (.location _returnvalue) (.rotation _returnvalue) "1.000000,1.000000,1.000000")))))))

(fn ConstructionScript)