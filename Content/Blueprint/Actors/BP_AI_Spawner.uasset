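; BP_AI_Spawner is an interactable actor that spawns an AI running the BT_EnnemyPuces behavior tree at its DestinationSpawn location.
; Its Interact event is gated by the HasSpawned flag, which a Delay clears after a short cooldown so spawning can repeat.
; A Box overlap shows the Widget while a CharacterMaster is inside and hides it when that character leaves.
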(event OnComponentBeginOverlap(Box)
  (params (OverlappedComponent :type Primitive%20Component%20Object%20Reference) (OtherActor :type Actor%20Object%20Reference) (OtherComp :type Primitive%20Component%20Object%20Reference) (OtherBodyIndex :type Integer) (bFromSweep :type Boolean) (SweepResult :type Hit%20Result%20Structure%20%28by%20ref%29))
  (Utilities|Casting|CastToCharacterMaster OtherActor)
  (Rendering|SetVisibility (Variables|Default|GetWidget) true false))

(event OnComponentEndOverlap(Box)
  (params (OverlappedComponent :type Primitive%20Component%20Object%20Reference) (OtherActor :type Actor%20Object%20Reference) (OtherComp :type Primitive%20Component%20Object%20Reference) (OtherBodyIndex :type Integer))
  (Utilities|Casting|CastToCharacterMaster OtherActor)
  (Rendering|SetVisibility (Variables|Default|GetWidget) false false))

(event EventBeginPlay)

(event Collision|EventActorBeginOverlap
  (params (OtherActor :type Actor%20Object%20Reference)))

(event EventTick
  (params (DeltaSeconds :type Float%20%28single-precision%29)))

(event EventInteract
  (if (not (Variables|Default|GetHasSpawned))
    (Variables|Default|SetHasSpawned true)
    (AI|SpawnAIFromClass 0 "/Game/Blueprint/AI/AI_Puces/BehaviourTree/BT_EnnemyPuces.BT_EnnemyPuces" (.location (Transformation|GetWorldTransform (Variables|Default|GetDestinationSpawn))) "0, 0, 0" false 0)
    (Utilities|FlowControl|Delay 1e+01)
    (Variables|Default|SetHasSpawned false)))

(fn ConstructionScript)