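; Actor that moves a Target actor along a spline at a fixed rotation, in world space.
; Tick sets the MoveAlongSpline timeline's play rate from the reciprocal of MoveAlongSplineTime and calls Play every frame.
; Each timeline update maps the curve value to a distance along the spline length and places Target there.
; StopSplineMovement disables Tick, so playback is not re-triggered, and stops the timeline.
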(event Custom|StopSplineMovement
  (Actor|Tick|SetActorTickEnabled false)
  (bind _spline (Timeline|MoveAlongSpline Stop)
    (:Update
      (Transformation|SetActorTransform (Variables|Default|GetTarget) (Math|Transform|MakeTransform (Spline|GetLocationatDistanceAlongSpline (Variables|Default|GetSpline) (Math|Float|Lerp 0.0 (Spline|GetSplineLength (Variables|Default|GetSpline)) _spline) "World") "-90.000000,0.000000,0.000000" "1.000000,1.000000,1.000000")))))

(event EventBeginPlay)

(event Collision|EventActorBeginOverlap
  (params (OtherActor :type Actor%20Object%20Reference)))

(event EventTick
  (params (DeltaSeconds :type Float%20%28single-precision%29))
  (Components|Timeline|SetPlayRate (Variables|Default|GetMoveAlongSpline) (/ 1.0 (Variables|Default|GetMoveAlongSplineTime)))
  (bind _spline (Timeline|MoveAlongSpline Play)
    (:Update
      (Transformation|SetActorTransform (Variables|Default|GetTarget) (Math|Transform|MakeTransform (Spline|GetLocationatDistanceAlongSpline (Variables|Default|GetSpline) (Math|Float|Lerp 0.0 (Spline|GetSplineLength (Variables|Default|GetSpline)) _spline) "World") "-90.000000,0.000000,0.000000" "1.000000,1.000000,1.000000")))))

(fn ConstructionScript)