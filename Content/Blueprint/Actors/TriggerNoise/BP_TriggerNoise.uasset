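; A one-shot trigger actor that alerts spawners and makes noise at the player's position when a CharacterMaster enters its collision box.
; On first overlap it enables hearing on the referenced spawners, clears their StartClosed flag and swings a referenced spotlight to a fixed yaw via timeline.
; After the light's rotation time, it reports a noise event at the character's current location three times in quick succession.
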(event OnComponentBeginOverlap(CollisionBox)
  (params (OverlappedComponent :type Primitive%20Component%20Object%20Reference) (OtherActor :type Actor%20Object%20Reference) (OtherComp :type Primitive%20Component%20Object%20Reference) (OtherBodyIndex :type Integer) (bFromSweep :type Boolean) (SweepResult :type Hit%20Result%20Structure%20%28by%20ref%29))
  (bind _ascharacter_master (Utilities|Casting|CastToCharacterMaster OtherActor))
  (Variables|Default|Setas%20Character%20Master _ascharacter_master)
  (Utilities|FlowControl|DoOnce false
    (:Completed
      (for _array_element (Variables|Default|GetBp_SpawnerRef)
        (Default|EnableHearing _array_element)
        (Variables|/Game/Blueprint/Actors/Spawner/BP_Spawner.BP_Spawner_C|SetStart%20Closed _array_element false))
      (Utilities|FlowControl|Sequence
        (:then_0
          (CallFunction|RotateSpotLight))
        (:then_1
          (Utilities|FlowControl|Delay (Variables|Default|GetlightRotTime))
          (CallFunction|ReportNoise))))))

(event Custom|ReportNoise
  (Class|AISenseHearing|ReportNoiseEvent (Transformation|GetActorLocation (Variables|Default|Getas%20Character%20Master)) 1.0 (Variables|Default|Getas%20Character%20Master) 2e+03 "None")
  (Utilities|FlowControl|Delay 0.2)
  (Math|Integer|IncrementInt (Variables|Default|GetnumberOfRepetition)
    (:%20%20
      (if (< (Variables|Default|GetnumberOfRepetition) 3)
        (CallFunction|ReportNoise)))))

(event Custom|RotateSpotLight
  (Components|Timeline|SetPlayRate (Variables|Default|GetRotationLight) (/ 1.0 (Variables|Default|GetlightRotTime)))
  (bind _rotation (Timeline|RotationLight PlayFromStart)
    (:Update
      (Transformation|SetActorRotation (Variables|Default|GetspotLightRef) (Math|Rotator|MakeRotator 0.0 0.0 (Math|Float|Lerp (.yaw (Transformation|GetActorRotation (Variables|Default|GetspotLightRef))) 1.7e+02 _rotation))))))

(event EventBeginPlay)

(fn ConstructionScript)