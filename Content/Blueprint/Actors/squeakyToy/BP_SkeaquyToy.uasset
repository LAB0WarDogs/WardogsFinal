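; Squeaky toy distraction actor that squeaks and emits an AI noise event as soon as it spawns.
; On BeginPlay it borrows the NoiseArea of BP_SecondChara, moving it to the toy, showing it and enlarging it in X and Y.
; It plays the sound and reports noise with that character as instigator.
; After a short delay it returns the area's position and scale, leaves it visible, and destroys itself.
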(event EventBeginPlay
  (bind _returnvalue (Transformation|GetActorLocation))
  (Utilities|FlowControl|Sequence
    (:then_0
      (bind _returnvalue_2 (Actor|GetActorOfClass "/Game/Blueprint/Character/BP_SecondChara.BP_SecondChara_C"))
      (bind _output_get (Variables|Default|SetSecondCharaRef _returnvalue_2))
      (Variables|Default|SetNoise%20Area (Variables|/Game/Blueprint/Character/CharacterMaster.CharacterMaster_C|GetNoiseArea _output_get))
      (Variables|Default|SetOriginalWorldScale (Transformation|GetWorldScale (Variables|/Game/Blueprint/Character/CharacterMaster.CharacterMaster_C|GetNoiseArea _output_get)))
      (Transformation|SetWorldLocation (Variables|Default|GetNoise%20Area) (Transformation|GetActorLocation) false false)
      (Rendering|SetVisibility (Variables|/Game/Blueprint/Character/CharacterMaster.CharacterMaster_C|GetNoiseArea _output_get) true false)
      (Transformation|SetWorldScale3D (Variables|/Game/Blueprint/Character/CharacterMaster.CharacterMaster_C|GetNoiseArea _output_get) (Math|Vector|MakeVector (+ (.x (Transformation|GetWorldScale (Variables|/Game/Blueprint/Character/CharacterMaster.CharacterMaster_C|GetNoiseArea _output_get))) 2e+01) (+ (.y (Transformation|GetWorldScale (Variables|/Game/Blueprint/Character/CharacterMaster.CharacterMaster_C|GetNoiseArea _output_get))) 2e+01) (.z (Transformation|GetWorldScale (Variables|/Game/Blueprint/Character/CharacterMaster.CharacterMaster_C|GetNoiseArea _output_get))))))
    (:then_1
      (Audio|PlaySoundatLocation "/Game/Sound/SqueakyToy/SqueatyToy_Cue.SqueatyToy_Cue" _returnvalue "0, 0, 0" 1.0 1.0 0.0 0 0 0 0)
      (Class|AISenseHearing|ReportNoiseEvent _returnvalue 1.0 (Variables|Default|GetSecondCharaRef) 2e+03 "None")
      (Utilities|FlowControl|Delay 1.0)
      (Transformation|SetWorldLocation (Variables|Default|GetNoise%20Area) (Transformation|GetActorLocation (Variables|Default|GetSecondCharaRef)) false false)
      (Transformation|SetWorldScale3D (Variables|Default|GetNoise%20Area) (Variables|Default|GetOriginalWorldScale))
      (Actor|DestroyActor))))

(fn ConstructionScript)