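; BP_Trap is a placed trap actor for the player's trap skill that paralyses AI walking into it.
; On trigger, it paralyses the victim through its AI controller, starts the skill cooldown, destroys itself and sphere-overlaps for damageable AI to paralyse more briefly, with debug drawing.
; The player's overlap toggles a widget, and Interact cancels the skill and removes the trap.
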(event OnComponentBeginOverlap(Box)
  (params (OverlappedComponent :type Primitive%20Component%20Object%20Reference) (OtherActor :type Actor%20Object%20Reference) (OtherComp :type Primitive%20Component%20Object%20Reference) (OtherBodyIndex :type Integer) (bFromSweep :type Boolean) (SweepResult :type Hit%20Result%20Structure%20%28by%20ref%29))
  (bind _returnvalue (Transformation|GetActorLocation))
  (bind _thirdchararef (Variables|Default|GetThirdCharaRef))
  (bind _returnvalue_2 (+ _returnvalue "0, 0, 0"))
  (bind _bp_trap (Variables|/Game/Blueprint/Character/BP_ThirdChara.BP_ThirdChara_C|GetBP_Trap _thirdchararef))
  (Utilities|Casting|CastToBP_ThirdChara OtherActor
    (:then
      (Rendering|SetVisibility (Variables|Default|GetWidget) true false))
    (:CastFailed
      (bind _asbp_ai_master (Utilities|Casting|CastToBP_AI_Master OtherActor))
      (bind _asbp_ai_controller_master (Utilities|Casting|CastToBP_AiControllerMaster (AI|GetAIController _asbp_ai_master)))
      (Default|Paralysed _asbp_ai_controller_master 1e+01 (Variables|/Game/Blueprint/AI/AI_Puces/AIController/BP_AiControllerMaster.BP_AiControllerMaster_C|GetBTAsset _asbp_ai_controller_master))
      (Utilities|FlowControl|Sequence
        (:then_0
          (Default|CoolDown _bp_trap)
          (Variables|/Game/Blueprint/SkiilsActorComponent/BP_TrapSkills.BP_TrapSkills_C|SetTrapHasBeenSet _bp_trap false)
          (Actor|DestroyActor))
        (:then_1
          (Rendering|Debug|DrawDebugSphere _returnvalue_2 (Variables|Default|GetRadius) 12 "(R=1.000000,G=0.000000,B=0.000000,A=1.000000)" 2.0)
          (bind _outactors (Collision|SphereOverlapActors _returnvalue_2 (Variables|Default|GetRadius) (Variables|Default|GetObject%20Types) 0))
          (for _array_element _outactors
            (if (Utilities|DoesObjectImplementInterface _array_element "/Game/Blueprint/Interface/BPI_Damageable.BPI_Damageable_C")
              (bind _asbp_ai_master_2 (Utilities|Casting|CastToBP_AI_Master _array_element))
              (bind _asbp_ai_controller_master_2 (Utilities|Casting|CastToBP_AiControllerMaster (AI|GetAIController _asbp_ai_master_2)))
              (Default|Paralysed _asbp_ai_controller_master_2 8.0 (Variables|/Game/Blueprint/AI/AI_Puces/AIController/BP_AiControllerMaster.BP_AiControllerMaster_C|GetBTAsset _asbp_ai_controller_master_2)))))))))

(event OnComponentEndOverlap(Box)
  (params (OverlappedComponent :type Primitive%20Component%20Object%20Reference) (OtherActor :type Actor%20Object%20Reference) (OtherComp :type Primitive%20Component%20Object%20Reference) (OtherBodyIndex :type Integer))
  (Utilities|Casting|CastToBP_ThirdChara OtherActor)
  (Rendering|SetVisibility (Variables|Default|GetWidget) false false))

(event EventInteract
  (bind _thirdchararef (Variables|Default|GetThirdCharaRef))
  (bind _bp_trap (Variables|/Game/Blueprint/Character/BP_ThirdChara.BP_ThirdChara_C|GetBP_Trap _thirdchararef))
  (Variables|/Game/Blueprint/SkiilsActorComponent/BP_TrapSkills.BP_TrapSkills_C|SetTrapHasBeenSet _bp_trap false)
  (Default|CancelTrapSkill _bp_trap)
  (Actor|DestroyActor))

(event EventBeginPlay
  (bind _returnvalue (Actor|GetActorOfClass "/Game/Blueprint/Character/BP_ThirdChara.BP_ThirdChara_C"))
  (Variables|Default|SetThirdCharaRef _returnvalue))

(fn ConstructionScript)