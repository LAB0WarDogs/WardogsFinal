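; Test NPC that starts a dialogue through its BP_Test_AI controller when a CharacterMaster overlaps it.
; On BeginPlay it passes its dialogue tree to that controller and hides its widget.
; Actor overlap or the ForceDialogue event calls StartDialogue on the controller.
; When a CharacterMaster leaves the box, the box's collision is disabled, so that trigger does not fire again.
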(event OnComponentEndOverlap(Box)
  (params (OverlappedComponent :type Primitive%20Component%20Object%20Reference) (OtherActor :type Actor%20Object%20Reference) (OtherComp :type Primitive%20Component%20Object%20Reference) (OtherBodyIndex :type Integer))
  (Utilities|Casting|CastToCharacterMaster OtherActor)
  (Collision|SetCollisionEnabled (Variables|Default|GetBox) "NoCollision"))

(event Custom|ForceDialogue
  ;[0 1 0] Interact
  (bind _asbp_test_ai (Utilities|Casting|CastToBP_Test_AI (AI|GetAIController self)))
  (Default|StartDialogue _asbp_test_ai))

(event Collision|EventActorBeginOverlap
  (params (OtherActor :type Actor%20Object%20Reference))
  ;[0 1 0] Interact
  (Utilities|Casting|CastToCharacterMaster OtherActor)
  (bind _asbp_test_ai (Utilities|Casting|CastToBP_Test_AI (AI|GetAIController self)))
  (Default|StartDialogue _asbp_test_ai))

(event EventBeginPlay
  ;[0 1 0] Set Tree used
  (bind _asbp_test_ai (Utilities|Casting|CastToBP_Test_AI (AI|GetAIController self)))
  (Variables|/Game/Blueprint/Actors/testDialogue/BP_Test_AI.BP_Test_AI_C|SetDialogueTree _asbp_test_ai (Variables|Default|GetDialogeTree))
  (Rendering|SetVisibility (Variables|Default|GetWidget) false false))

(fn ConstructionScript)