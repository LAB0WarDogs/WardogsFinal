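; BP_Spawner is an actor that spawns a BP_AI_PucesSentinel at its own location when its AIPerception component reports a target update.
; An EnableHearing event turns on the hearing sense, and a DoOnce gates spawning.
; Each sentinel runs BT_Sentinel and receives the spawner's patrol path and a fixed PressesNeeded value.
; With MultipleRespawn set, the gate resets after DelayBetweenSpawn, allowing another perception update to spawn again.
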(event OnTargetPerceptionUpdated(AIPerception)
  (params (Actor :type Actor%20Object%20Reference) (Stimulus :type AI%20Stimulus%20Structure))
  (Utilities|FlowControl|DoOnce (Variables|Default|GetStart%20Closed)
    (:Completed
      (bind _returnvalue (AI|SpawnAIFromClass "/Game/Blueprint/AI/AI_Puces/AiCharacter/BP_AI_PucesSentinel.BP_AI_PucesSentinel_C" "/Game/Blueprint/AI/AI_Puces/BehaviourTree/BT_Sentinel.BT_Sentinel" (Transformation|GetActorLocation self) "0, 0, 0" false 0))
      (bind _asbp_ai_puces_sentinel (Utilities|Casting|CastToBP_AI_PucesSentinel _returnvalue))
      (Variables|/Game/Blueprint/AI/AI_Puces/AiCharacter/BP_AI_Master.BP_AI_Master_C|SetPatrolPath _asbp_ai_puces_sentinel (Variables|Default|GetpatrolPhat))
      (Variables|/Game/Blueprint/AI/AI_Puces/AiCharacter/BP_AI_PucesSentinel.BP_AI_PucesSentinel_C|SetPressesNeeded _asbp_ai_puces_sentinel 5.0)
      (if (Variables|Default|GetMultipleRespawn)
        (Utilities|FlowControl|Delay (Variables|Default|GetDelayBetweenSpawn))
        (CallFunction|ResetDoOnce)))))

(event Custom|EnableHearing
  (Class|AIPerceptionComponent|SetSenseEnabled (Variables|Default|GetAIPerception) "/Script/AIModule.AISense_Hearing" true))

(event Custom|ResetDoOnce
  (Utilities|FlowControl|DoOnce (Variables|Default|GetStart%20Closed)) ; enters at Reset
)

(fn ConstructionScript)