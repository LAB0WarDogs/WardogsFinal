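; Dissolve mask actor that follows the active character's camera and defines the area used by dissolve materials.
; Shortly after BeginPlay it takes BP_FirstChara's camera, then switches to the current character's camera whenever the GameMode broadcasts a character switch.
; Each tick it sits ahead of that camera and writes its mesh's location and scale to MPC_DIssolveArea.
; The construction script writes the same parameters, so the collection also updates in the editor.
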(event Custom|CustomEvent_1
  ;[0 0 1] Setup
  (bind _asgame_mode_wardogs (CallFunction|GetGameMode))
  (bind _ascharacter_master (Utilities|Casting|CastToCharacterMaster (Utilities|Array|Get(acopy) (Variables|/Game/Blueprint/GameMode/GameModeWardogs.GameModeWardogs_C|GetArrayCharaRef _asgame_mode_wardogs) (Variables|/Game/Blueprint/GameMode/GameModeWardogs.GameModeWardogs_C|GetCharaIndex _asgame_mode_wardogs))))
  (Variables|Default|SetFollowedCamera (Variables|/Game/Blueprint/Character/CharacterMaster.CharacterMaster_C|GetCamera _ascharacter_master)))

(event EventBeginPlay
  ;[0 0 1] Setup
  (Utilities|FlowControl|Delay 0.2)
  (Utilities|FlowControl|Sequence
    (:then_0
      (bind _returnvalue (Actor|GetActorOfClass "/Game/Blueprint/Character/BP_FirstChara.BP_FirstChara_C"))
      (bind _output_get (Variables|Default|SetFollowedCamera (Variables|/Game/Blueprint/Character/CharacterMaster.CharacterMaster_C|GetCamera _returnvalue)))
      (Transformation|SetActorLocation (Transformation|GetWorldLocation _output_get) false false))
    (:then_1
      (bind _asgame_mode_wardogs (CallFunction|GetGameMode))
      (EventDispatchers|BindEventtoCharacterasBeenSwitched _asgame_mode_wardogs (delegate Custom|CustomEvent_1)))))

(event EventTick
  (params (DeltaSeconds :type Float%20%28single-precision%29))
  (bind _staticmesh (Variables|Default|GetStaticMesh))
  ;[0 0 1] Tick
  (bind _followedcamera (Variables|Default|GetFollowedCamera)
    (:then
      (Transformation|SetActorLocation (+ (* (Math|Vector|GetForwardVector _followedcamera) "700.000000,700.000000,800.000000") (Transformation|GetWorldLocation _followedcamera)) false false)
      (Rendering|Material|SetVectorParameterValue "/Game/Material/DissolveMask/MPC_DIssolveArea.MPC_DIssolveArea" "Location" (Math|Conversions|ToLinearColor(Vector) (Transformation|GetWorldLocation _staticmesh)) :!class /Script/Engine.KismetMaterialLibrary)
      (Rendering|Material|SetVectorParameterValue "/Game/Material/DissolveMask/MPC_DIssolveArea.MPC_DIssolveArea" "Scale" (Math|Conversions|ToLinearColor(Vector) (Transformation|GetWorldScale _staticmesh)) :!class /Script/Engine.KismetMaterialLibrary))
    (:else)))

(fn ConstructionScript
  (bind _staticmesh (Variables|Default|GetStaticMesh))
  (Rendering|Material|SetVectorParameterValue "/Game/Material/DissolveMask/MPC_DIssolveArea.MPC_DIssolveArea" "Location" (Math|Conversions|ToLinearColor(Vector) (Transformation|GetWorldLocation _staticmesh)) :!class /Script/Engine.KismetMaterialLibrary)
  (Rendering|Material|SetVectorParameterValue "/Game/Material/DissolveMask/MPC_DIssolveArea.MPC_DIssolveArea" "Scale" (Math|Conversions|ToLinearColor(Vector) (Transformation|GetWorldScale _staticmesh)) :!class /Script/Engine.KismetMaterialLibrary))