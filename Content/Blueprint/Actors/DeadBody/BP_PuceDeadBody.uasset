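; Dead body actor for a Puce that can revive as a sentinel AI unless it takes damage first.
; On initialization with Respawn, it waits, then spawns BP_AI_PucesSentinel at the body, passes on the patrol path and destroys itself.
; Damage marks it permanently dead; this or a non-respawn initialization swaps to the dead material and makes the box ignore a custom trace channel.
; Initialization also re-records the body's location after a delay.
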(event Custom|CheckDeadBody)

(event Custom|InitializationDeadBody
  (params (Vector3 :type Vector) (Actor :type Actor%20Object%20Reference) (Respawn :type Boolean))
  (Variables|Default|SetPuceOwner Actor)
  (Variables|Default|SetActorLocation Vector3)
  (Utilities|FlowControl|Sequence
    (:then_0
      (if Respawn
        (Utilities|FlowControl|Delay (Variables|Default|GetWaitToRespaw))
        (if (not (Variables|Default|GetMorte))
          (bind _returnvalue (AI|SpawnAIFromClass "/Game/Blueprint/AI/AI_Puces/AiCharacter/BP_AI_PucesSentinel.BP_AI_PucesSentinel_C" "/Game/Blueprint/AI/AI_Puces/BehaviourTree/BT_Sentinel.BT_Sentinel" (Transformation|GetWorldLocation (Variables|Default|Getpuce)) "0, 0, 0" true 0))
          (bind _asbp_ai_puces_sentinel (Utilities|Casting|CastToBP_AI_PucesSentinel _returnvalue))
          (Variables|/Game/Blueprint/AI/AI_Puces/AiCharacter/BP_AI_Master.BP_AI_Master_C|SetPatrolPath _asbp_ai_puces_sentinel (Variables|Default|GetPatroPath))
          (Variables|/Game/Blueprint/AI/AI_Puces/AiCharacter/BP_AI_PucesSentinel.BP_AI_PucesSentinel_C|SetPressesNeeded _asbp_ai_puces_sentinel 5.0)
          (Pawn|SpawnDefaultController _asbp_ai_puces_sentinel)
          (Actor|DestroyActor))
        (else
          (Rendering|Material|SetMaterial (Variables|Default|Getpuce) 1 "/Game/Material/PUCES/PUCES_GIROMorte.PUCES_GIROMorte")
          (Collision|SetCollisionResponsetoChannel (Variables|Default|GetBox) "ECC_GameTraceChannel5" "ECR_Ignore"))))
    (:then_1
      (Utilities|FlowControl|Delay (Variables|Default|GetDelayChercheZone))
      (Variables|Default|SetActorLocation (Transformation|GetActorLocation self)))))

(event EventTakeDamage
  (params (Damage :type Float%20%28double-precision%29))
  (Variables|Default|SetMorte true)
  (Rendering|Material|SetMaterial (Variables|Default|Getpuce) 1 "/Game/Material/PUCES/PUCES_GIROMorte.PUCES_GIROMorte")
  (Collision|SetCollisionResponsetoChannel (Variables|Default|GetBox) "ECC_GameTraceChannel5" "ECR_Ignore"))

(fn ConstructionScript)