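; One-shot trigger zone that enables or disables a character's three skills when a CharacterMaster enters its box.
; Its three Activate flags are written to the CanUse skill properties of the overlapping character, or of its First, Second and Third characters when ActivateAllSkills is set.
; Each write refreshes InGameUI through Switch, using the GameMode's current character index.
; The actor destroys itself when a CharacterMaster leaves the box.
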(event OnComponentBeginOverlap(Box)
  (params (OverlappedComponent :type Primitive%20Component%20Object%20Reference) (OtherActor :type Actor%20Object%20Reference) (OtherComp :type Primitive%20Component%20Object%20Reference) (OtherBodyIndex :type Integer) (bFromSweep :type Boolean) (SweepResult :type Hit%20Result%20Structure%20%28by%20ref%29))
  (bind _activatefirstskill (Variables|Default|GetActivateFirstSkill))
  (bind _activatesecondskill (Variables|Default|GetActivateSecondSkill))
  (bind _activatethirdskill (Variables|Default|GetActivateThirdSkill))
  (bind _ascharacter_master (Utilities|Casting|CastToCharacterMaster OtherActor))
  (if (Variables|Default|GetActivateAllSkills)
    (Utilities|FlowControl|Sequence
      (:then_0
        (Variables|/Game/Blueprint/Character/CharacterMaster.CharacterMaster_C|SetCanUseFirstSkill (Variables|/Game/Blueprint/Character/CharacterMaster.CharacterMaster_C|GetFirstChara _ascharacter_master) _activatefirstskill)
        (Variables|/Game/Blueprint/Character/CharacterMaster.CharacterMaster_C|SetCanUseSecondarySkill (Variables|/Game/Blueprint/Character/CharacterMaster.CharacterMaster_C|GetFirstChara _ascharacter_master) _activatesecondskill)
        (Variables|/Game/Blueprint/Character/CharacterMaster.CharacterMaster_C|SetCanUseThirdSkill (Variables|/Game/Blueprint/Character/CharacterMaster.CharacterMaster_C|GetFirstChara _ascharacter_master) _activatethirdskill))
      (:then_1
        (Variables|/Game/Blueprint/Character/CharacterMaster.CharacterMaster_C|SetCanUseFirstSkill (Variables|/Game/Blueprint/Character/CharacterMaster.CharacterMaster_C|GetSecondChara _ascharacter_master) _activatefirstskill)
        (Variables|/Game/Blueprint/Character/CharacterMaster.CharacterMaster_C|SetCanUseSecondarySkill (Variables|/Game/Blueprint/Character/CharacterMaster.CharacterMaster_C|GetSecondChara _ascharacter_master) _activatesecondskill)
        (Variables|/Game/Blueprint/Character/CharacterMaster.CharacterMaster_C|SetCanUseThirdSkill (Variables|/Game/Blueprint/Character/CharacterMaster.CharacterMaster_C|GetSecondChara _ascharacter_master) _activatethirdskill))
      (:then_2
        (Variables|/Game/Blueprint/Character/CharacterMaster.CharacterMaster_C|SetCanUseFirstSkill (Variables|/Game/Blueprint/Character/CharacterMaster.CharacterMaster_C|GetThirdChara _ascharacter_master) _activatefirstskill)
        (Variables|/Game/Blueprint/Character/CharacterMaster.CharacterMaster_C|SetCanUseSecondarySkill (Variables|/Game/Blueprint/Character/CharacterMaster.CharacterMaster_C|GetThirdChara _ascharacter_master) _activatesecondskill)
        (Variables|/Game/Blueprint/Character/CharacterMaster.CharacterMaster_C|SetCanUseThirdSkill (Variables|/Game/Blueprint/Character/CharacterMaster.CharacterMaster_C|GetThirdChara _ascharacter_master) _activatethirdskill)))
    (else
      (Variables|/Game/Blueprint/Character/CharacterMaster.CharacterMaster_C|SetCanUseFirstSkill _ascharacter_master (Variables|Default|GetActivateFirstSkill))
      (Variables|/Game/Blueprint/Character/CharacterMaster.CharacterMaster_C|SetCanUseSecondarySkill _ascharacter_master (Variables|Default|GetActivateSecondSkill))
      (Variables|/Game/Blueprint/Character/CharacterMaster.CharacterMaster_C|SetCanUseThirdSkill _ascharacter_master (Variables|Default|GetActivateThirdSkill))))
  (bind _asgame_mode_wardogs (CallFunction|GetGameMode))
  (Default|Switch (Variables|/Game/Blueprint/Character/CharacterMaster.CharacterMaster_C|GetIn%20Game%20UI _ascharacter_master) (Variables|/Game/Blueprint/GameMode/GameModeWardogs.GameModeWardogs_C|GetCharaIndex _asgame_mode_wardogs) (Variables|Default|GetActivateFirstSkill) (Variables|Default|GetActivateSecondSkill) (Variables|Default|GetActivateThirdSkill)))

(event OnComponentEndOverlap(Box)
  (params (OverlappedComponent :type Primitive%20Component%20Object%20Reference) (OtherActor :type Actor%20Object%20Reference) (OtherComp :type Primitive%20Component%20Object%20Reference) (OtherBodyIndex :type Integer))
  (Utilities|Casting|CastToCharacterMaster OtherActor)
  (Actor|DestroyActor))

(fn ConstructionScript)